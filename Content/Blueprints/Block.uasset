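; Grid block actor for a roguelike building game that can become stone, grass or water, or host a fireplace that periodically adds Flame to the controller.
; Cursor hover drives selection and gated placement previews, with stone snapped to the hit normal.
; One reversible timeline moves rising and falling blocks, with Niagara falling effects.
; Line traces update covered blocks below, count neighbours for NearFall and find same-type neighbours for DirectionButton clicks.
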(event `On_Create`
  (bind _returnvalue (`SceneComponent.K2_GetComponentLocation` (`self.BlockMesh`)))
  (set `self.World_Pos` (`self.K2_GetActorLocation`))
  (`ActorComponent.SetActive` (`self.Falling_System`) (== (`self.Z_pos`) 0) true)
  (`|ExecutionSequence`
    (:`then_0`
      (bind _asdirection_button (cast `/Game/Interface/DirectionButton` (`WidgetComponent.GetWidget` (`self.Direction_Button`))))
      (set `/Game/Interface/DirectionButton.Owner` self _asdirection_button))
    (:`then_1`
      (`SceneComponent.SetVisibility` (`self.grass_bunch1`) false false)
      (`SceneComponent.SetVisibility` (`self.grass_bunch2`) false false)
      (`SceneComponent.SetVisibility` (`self.grass_bunch3`) false false)
      (`SceneComponent.SetVisibility` (`self.Water`) false false)
      (bind _outhit (`KismetSystemLibrary.LineTraceSingle` _returnvalue (+ _returnvalue (0.0 0.0 -300.0)) "TraceTypeQuery1"))
      (bind _asblock (cast `/Game/Blueprints/Block` (`.HitActor` (`GameplayStatics.BreakHitResult` _outhit))))
      (`self.Clear` _asblock)
      (`self.Set_Z_Covered_Z` _asblock false))))

(event `Force_Select`
  (bind _returnvalue (`GameplayStatics.GetPlayerController` 0))
  (bind _returnvalue_2 (and (`|EnumEquality` (`self.Block_Type`) "NewEnumerator0") (not (`self.Z_covered`))))
  ;[1 1 1] Overlay and selection
  (for _array_element (`/Game/Blueprints/BlockGridGenerator.Blocks_Array` (`self.OwningGrid`))
    (`self.Force_Deselect` _array_element))
  (`SceneComponent.SetVisibility` (`self.SelectionMark1`) (and (not (`self.Falling`)) (not (`self.Z_covered`)) (`|EnumEquality` (`/Game/Blueprints/RoguelikeController.Active_Block_Type` (stale `self.BlockMesh.OnBeginCursorOver` _asroguelike_controller)) "NewEnumerator3")) false :!label _label)
  (goto _label_2 :!via `Open`))

(event `Update_Preview`
  (bind _returnvalue (`GameplayStatics.GetPlayerController` 0))
  (bind _returnvalue_2 (and (`|EnumEquality` (`self.Block_Type`) "NewEnumerator0") (not (`self.Z_covered`))))
  (`/Engine/EditorBlueprintResources/StandardMacros.Gate` true :!label _label_2
    (:`Exit`
      (bind _asroguelike_controller (cast `/Game/Blueprints/RoguelikeController` _returnvalue))
      (switch `/Game/Blueprints/Buildable_Objects/Block_Type` (`/Game/Blueprints/RoguelikeController.Active_Block_Type` _asroguelike_controller)
        (:`NewEnumerator0`
          (bind _output_get (set `self.Preview_Normal_Vector` (`.Normal` (`GameplayStatics.BreakHitResult` (`PlayerController.GetHitResultUnderCursorByChannel` _returnvalue "TraceTypeQuery2" true)))))
          (`SceneComponent.SetVisibility` (`self.Stone_Preview`) true false)
          (`|ExecutionSequence`
            (:`then_0`
              (if (> (`KismetMathLibrary.Abs` (.x _output_get)) 0.9)
                (set `self.Preview_Vector` (`KismetMathLibrary.MakeVector` (`KismetMathLibrary.SafeDivide` (.x _output_get) (`KismetMathLibrary.Abs` (.x _output_get)))))
                (`SceneComponent.K2_SetRelativeLocation` (`self.Stone_Preview`) (* (`self.Preview_Vector`) 100) false false :!label _label_3)))
            (:`then_1`
              (if (> (`KismetMathLibrary.Abs` (.y _output_get)) 0.9)
                (set `self.Preview_Vector` (`KismetMathLibrary.MakeVector` 0.0 (`KismetMathLibrary.SafeDivide` (.y _output_get) (`KismetMathLibrary.Abs` (.y _output_get)))))
                (goto _label_3)))
            (:`then_2`
              (if (> (`KismetMathLibrary.Abs` (.z _output_get)) 0.9)
                (set `self.Preview_Vector` (`KismetMathLibrary.MakeVector` 0.0 0.0 (select `bool` (and (`|EnumEquality` (`self.Block_Type`) "NewEnumerator0") (not (`self.Z_covered`))) :`true` (`KismetMathLibrary.SafeDivide` (.z _output_get) (`KismetMathLibrary.Abs` (.z _output_get))))))
                (goto _label_3)))))
        (:`NewEnumerator1`
          (if _returnvalue_2
            (`SceneComponent.SetHiddenInGame` (`self.Water_Preview`) false false)))
        (:`NewEnumerator2`
          (if _returnvalue_2
            (`SceneComponent.SetHiddenInGame` (`self.grass_preview1`) false false)
            (`SceneComponent.SetHiddenInGame` (`self.grass_preview2`) false false)
            (`SceneComponent.SetHiddenInGame` (`self.grass_preview3`) false false)))))))

(event `self.BlockMesh.OnBeginCursorOver`
  (params (TouchedComponent :type "PrimitiveComponent Object Reference"))
  ;[1 1 1] Overlay and selection
  (bind _asroguelike_controller (cast `/Game/Blueprints/RoguelikeController` (`GameplayStatics.GetPlayerController` 0)))
  (`/Engine/EditorBlueprintResources/StandardMacros.IsValid` (`/Game/Blueprints/RoguelikeController.Build_Position_Block` _asroguelike_controller)
    (:`Is Not Valid`
      (goto _label))))

(event `self.BlockMesh.OnEndCursorOver`
  (params (TouchedComponent :type "PrimitiveComponent Object Reference"))
  ;[1 1 1] Overlay and selection
  (bind _asroguelike_controller (cast `/Game/Blueprints/RoguelikeController` (`GameplayStatics.GetPlayerController` 0)))
  (`/Engine/EditorBlueprintResources/StandardMacros.IsValid` (`/Game/Blueprints/RoguelikeController.Build_Position_Block` _asroguelike_controller)
    (:`Is Not Valid`
      (`SceneComponent.SetVisibility` (`self.SelectionMark1`) false false :!label _label_4)
      (`SceneComponent.SetVisibility` (`self.Stone_Preview`) false false)
      (`SceneComponent.SetHiddenInGame` (`self.grass_preview1`) true false)
      (`SceneComponent.SetHiddenInGame` (`self.grass_preview2`) true false)
      (`SceneComponent.SetHiddenInGame` (`self.grass_preview3`) true false)
      (`SceneComponent.SetHiddenInGame` (`self.Water_Preview`) true false)
      (goto _label_2 :!via `Close`))))

(event `Force_Deselect`
  ;[1 1 1] Overlay and selection
  (goto _label_4))

(event `Dark_Focus`
  (`NiagaraFunctionLibrary.SpawnSystemAtLocation` "/Game/Effects/Abyss_Accumulation.Abyss_Accumulation" (`SceneComponent.K2_GetComponentLocation` (`self.BlockMesh`))))

(event `Occupy`
  (params (NewOccupy :type Boolean))
  (bind _output_get (set `self.Occupied` NewOccupy))
  (if _output_get
    _))

(event `Update_Falling_System`
  (params (Rotator :type "Rotator Structure") (Wing_Alpha :type "Float (double-precision)"))
  (bind _falling_system (`self.Falling_System`))
  (bind _returnvalue (`KismetArrayLibrary.Array_Length` (`PrimitiveComponent.GetOverlappingActors` (`self.Falling_Checker`) "Block_C")))
  (`SceneComponent.K2_SetWorldRotation` (`self.Falling_Scene`) Rotator false false)
  (`/Engine/EditorBlueprintResources/StandardMacros.Gate` false :!label _label_5
    (:`Exit`
      (`NiagaraComponent.SetNiagaraVariableFloat` _falling_system "CustomSpawnrate" (select `bool` (> _returnvalue 1) :`false` (select `bool` (> _returnvalue 0) :`false` 10.0 :`true` 5.0 :!type "Float (single-precision)")))
      (`NiagaraComponent.SetNiagaraVariableFloat` _falling_system "CustomMaxSpeed" (* Wing_Alpha 500.0))
      (`NiagaraComponent.SetNiagaraVariableVec2` _falling_system "CustomSpeedScale" (10.0 350.0)))))

(event `Stop_Falling_System`
  (goto _label_5 :!via `Close`))

(event `Rise`
  (params (Custom_Rate :type "Float (double-precision)" :default 0.5) (Height :type "Float (double-precision)" :default 200.0))
  (bind (_fall_rotator_roll _fall_rotator_pitch _fall_rotator_yaw) (`KismetMathLibrary.BreakRotator` (`self.Fall_Rotator`)))
  ;[1 1 1] Fall
  (set `self.Falling` true)
  (`self.Set_Z_Covered_Z` false)
  (if (`self.Falling`)
    (set `self.Have_Mass` (not (!= Custom_Rate 0.5)))
    (set `self.Fall_Pos` (+ (`self.World_Pos`) (`KismetMathLibrary.MakeVector` 0.0 0.0 Height)))
    (`TimelineComponent.SetPlayRate` (`self.Fall_Timeleine`) Custom_Rate)
    (bind (_direction _alpha) (`Timeline|Fall_Timeleine` :!via `PlayFromStart` :!label _label_6)
      (:`Update`
        (`self.K2_SetActorLocation` (`KismetMathLibrary.VLerp` (`self.World_Pos`) (`self.Fall_Pos`) _alpha))
        (if (`self.Falling`)
          (`SceneComponent.K2_AddRelativeRotation` (`self.BlockMesh`) (`KismetMathLibrary.MakeRotator` (/ _fall_rotator_roll 180.0) (/ _fall_rotator_pitch 180.0) (/ _fall_rotator_yaw 180.0)) false false)))
      (:`Finished`
        (switch `ETimelineDirection` _direction
          (:`Forward`
            (`self.Stop_Falling_System`)
            (`ActorComponent.Deactivate` (`self.Falling_System`)))
          (:`Backward`
            (`self.On_Create`)))))))

(event `Fall`
  ;[1 1 1] Fall
  (set `self.Occupied` true)
  (set `self.Have_Mass` false)
  (set `self.Falling` true)
  (set `self.Fall_Pos` (+ (`self.World_Pos`) (`KismetMathLibrary.MakeVector` (* (`KismetMathLibrary.RandomIntegerInRange` -2 2) 200.0) (* (`KismetMathLibrary.RandomIntegerInRange` -2 2) 200.0) 3000.0)))
  (`PrimitiveComponent.SetMaterial` (`self.BlockMesh`) 0 "/Game/Meshes/_Materials/Cubes/RedFullCubeMat.RedFullCubeMat")
  (`TimelineComponent.SetPlayRate` (`self.Fall_Timeleine`) (`KismetMathLibrary.RandomFloatInRange` 2.5 10.0))
  (`KismetSystemLibrary.Delay` 0.2)
  (goto _label_6 :!via `PlayFromStart`))

(event `Cancel_Fall`
  ;[1 1 1] Fall
  (`self.Set_Z_Covered_Z` true)
  (goto _label_6 :!via `Reverse`))

(event `Enable_Fireplce`
  ;[1 1 1] Fireplaces
  (set `self.Have_Fireplace` true)
  (set `self.Block_Type` "NewEnumerator3")
  (`SceneComponent.SetHiddenInGame` (`self.Fireplace`) false false)
  (set `self.Occupied` true)
  (`SceneComponent.K2_SetRelativeRotation` (`self.Fireplace_Scene`) (`KismetMathLibrary.MakeRotator` 0.0 0.0 (* (`KismetMathLibrary.RandomIntegerInRange` 0 3) 90.0)) false false)
  (`KismetSystemLibrary.Delay` (`KismetMathLibrary.RandomFloatInRange` 0.0 5.0))
  (`self.Enflame`))

(event `Set_Z_Covered_Z`
  (params (New_Z_Covered :type Boolean))
  (bind _returnvalue (`SceneComponent.K2_GetComponentLocation` (`self.BlockMesh`)))
  ;[1 1 1] Z Cover
  (bind _outhit (`KismetSystemLibrary.LineTraceSingle` _returnvalue (+ _returnvalue (0.0 0.0 -300.0)) "TraceTypeQuery1"))
  (bind _asblock (cast `/Game/Blueprints/Block` (`.HitActor` (`GameplayStatics.BreakHitResult` _outhit))))
  (set `/Game/Blueprints/Block.Z_covered` New_Z_Covered _asblock))

(event `Enflame`
  (bind _floating_flame (`self.Floating_Flame`))
  ;[1 1 1] Fireplaces
  (`KismetSystemLibrary.Delay` 10.0)
  (if (`self.Have_Fireplace`)
    (`ActorComponent.Activate` (`self.Flames_Burst`) false)
    (`|ExecutionSequence`
      (:`then_0`
        (bind _asroguelike_controller (cast `/Game/Blueprints/RoguelikeController` (`GameplayStatics.GetPlayerController` 0)))
        (`/Engine/EditorBlueprintResources/StandardMacros.IncrementInt` (`/Game/Blueprints/RoguelikeController.Flame` _asroguelike_controller)
          (:`  `
            (`self.Enflame`))))
      (:`then_1`
        (bind (_direction _pos) (`Timeline|Enflame_TM` :!via `PlayFromStart`)
          (:`Update`
            (`SceneComponent.K2_SetRelativeLocation` _floating_flame (`KismetMathLibrary.MakeVector` 0.0 0.0 (* _pos 900.0)) false false)
            (bind _returnvalue (- _pos 0.5))
            (bind _returnvalue_2 (- 1.1 (* _returnvalue _returnvalue 4.0)))
            (`SceneComponent.SetRelativeScale3D` _floating_flame (`KismetMathLibrary.MakeVector` _returnvalue_2 _returnvalue_2 _returnvalue_2))))))))

(event `GrowGrass`
  ;[1 1 1] Grass
  (`SceneComponent.SetVisibility` (`self.grass_bunch1`) true false)
  (`SceneComponent.SetVisibility` (`self.grass_bunch2`) true false)
  (`SceneComponent.SetVisibility` (`self.grass_bunch3`) true false)
  (`SceneComponent.K2_SetRelativeRotation` (`self.Grass_Scene`) (`KismetMathLibrary.MakeRotator` 0.0 0.0 (* (`KismetMathLibrary.RandomIntegerInRange` 0 3) 90.0)) false false)
  (`PrimitiveComponent.SetMaterial` (`self.BlockMesh`) 0 "/Game/Meshes/_Materials/Cubes/GrassFullCubeMat.GrassFullCubeMat")
  (set `self.Block_Type` "NewEnumerator2"))

(event `Check_Near`
  (bind _returnvalue (`SceneComponent.K2_GetComponentLocation` (`self.BlockMesh`)))
  ;[1 1 1] Check for near
  (set `self.Near_Blocks_Number` 0)
  (for _index (range 8)
    (bind _outhit (`KismetSystemLibrary.LineTraceSingle` (+ _returnvalue (0.0 0.0 500.0)) (+ _returnvalue (`KismetMathLibrary.GreaterGreater_VectorRotator` (250.0 0.0 0.0) (`KismetMathLibrary.MakeRotator` 0.0 0.0 (* _index 45.0)))) "TraceTypeQuery1"))
    (bind _asblock (cast `/Game/Blueprints/Block` (`.HitActor` (`GameplayStatics.BreakHitResult` _outhit))))
    (set `self.Near_Blocks_Number` (+ (`self.Near_Blocks_Number`) (`KismetMathLibrary.Conv_BoolToInt` (not (`/Game/Blueprints/Block.Falling` _asblock)))))))

(event `Add_Water`
  ;[1 1 1] Water
  (`SceneComponent.SetVisibility` (`self.Water`) true false)
  (set `self.Block_Type` "NewEnumerator1"))

(event `NearFall`
  (params (FallFactor :type Integer))
  ;[1 1 1] Check for near
  (if (and (<= (`self.Near_Blocks_Number`) FallFactor) (not (`self.Falling`)))
    (`self.Fall`)
    (`PrimitiveComponent.SetMaterial` (`self.BlockMesh`) 0 "/Game/Meshes/_Materials/Cubes/AngelFullCubeMat.AngelFullCubeMat")))

(event `Clear`
  (bind _flames_burst (`self.Flames_Burst`))
  ;[1 1 1] Clear
  (`SceneComponent.SetVisibility` (`self.Water`) false false)
  (`SceneComponent.SetVisibility` (`self.grass_bunch1`) false false)
  (`SceneComponent.SetVisibility` (`self.grass_bunch2`) false false)
  (`SceneComponent.SetVisibility` (`self.grass_bunch3`) false false)
  (`SceneComponent.SetVisibility` (`self.Fireplace`) false false)
  (set `self.Occupied` false)
  (`PrimitiveComponent.SetMaterial` (`self.BlockMesh`) 0 "/Game/Meshes/_Materials/Cubes/WhiteFullCubeMat.WhiteFullCubeMat")
  (if (`self.Have_Fireplace`)
    (`ActorComponent.Activate` _flames_burst false)
    (`NiagaraFunctionLibrary.SpawnSystemAtLocation` "/Game/Effects/Fireplace_Destrunction.Fireplace_Destrunction" (`SceneComponent.K2_GetComponentLocation` _flames_burst))
    (set `self.Block_Type` "NewEnumerator0")
    (bind _asroguelike_controller (cast `/Game/Blueprints/RoguelikeController` (`GameplayStatics.GetPlayerController` 0)))
    (set `/Game/Blueprints/RoguelikeController.Flame` (+ (`/Game/Blueprints/RoguelikeController.Flame` _asroguelike_controller) 10) _asroguelike_controller)
    (set `self.Have_Fireplace` false)))

(event `Avilible_For_Direction_Click`
  (params (Slot_N :type Integer))
  (bind _direction_button (`self.Direction_Button`))
  (`SceneComponent.K2_SetRelativeLocation` _direction_button (0.0 0.0 90.0) false false)
  (bind _asdirection_button (cast `/Game/Interface/DirectionButton` (`WidgetComponent.GetWidget` _direction_button)))
  (set `/Game/Interface/DirectionButton.Slot_N` Slot_N _asdirection_button))

(event `Unavilible_For_Direction_Click`
  (`SceneComponent.K2_SetRelativeLocation` (`self.Direction_Button`) (0.0 0.0 0.0) false false))

(fn `Find Near Blocks Same Type`
  (params (Size :type Integer) (Slot_N :type Integer))
  (returns (Result :type Boolean))
  (locals (Counter :type Integer))
  (bind _returnvalue (`SceneComponent.K2_GetComponentLocation` (`self.BlockMesh`)))
  (`/Game/Blueprints/BlockGridGenerator.After_Direction_Click` (`self.OwningGrid`))
  (if (== Size 1)
    (return true)
    (elif (== Size 2)
      (set `local.Counter` 0)
      (for _index (range 4)
        (bind _outhit (`KismetSystemLibrary.LineTraceSingle` (+ _returnvalue (0.0 0.0 500.0)) (+ _returnvalue (`KismetMathLibrary.GreaterGreater_VectorRotator` (250.0 0.0 0.0) (`KismetMathLibrary.MakeRotator` 0.0 0.0 (* _index 90.0)))) "TraceTypeQuery1"))
        (bind _asblock (cast `/Game/Blueprints/Block` (`.HitActor` (`GameplayStatics.BreakHitResult` _outhit))))
        (if (and (`|EnumEquality` (`/Game/Blueprints/Block.Block_Type` _asblock) (`self.Block_Type`)) (== (`/Game/Blueprints/Block.Z_pos` _asblock) (`self.Z_pos`)))
          (`/Engine/EditorBlueprintResources/StandardMacros.IncrementInt` (`local.Counter`)
            (:`  `
              (`self.Avilible_For_Direction_Click` _asblock Slot_N)))))
      (return (> (`local.Counter`) 0)))))

(fn `UserConstructionScript`)