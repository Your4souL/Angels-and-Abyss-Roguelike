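; Ray attack actor in the angel attack set that damages Abyss_Hand actors it touches, then destroys itself.
; The Attack event plays a slowed timeline that drives the cube's relative Z location, with destruction following a short delay after it finishes.
; Collision overlaps apply damage to the hand, directed away from ScalePoint1.
; Timeline-driven scaling of ScalePoint1 and the cube is disconnected, leaving the ScaleMultiplayer input without effect.
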(event `Attack`
  (params (Scale_Multiplayer :type "Float (double-precision)"))
  (`TimelineComponent.SetPlayRate` (`self.Attack_Timeline`) 0.5)
  (bind (_direction _scale _fade _position) (`Timeline|Attack_Timeline` :!via `PlayFromStart`)
    (:`Update`
      (`SceneComponent.K2_SetRelativeLocation` (`self.Cube`) (`KismetMathLibrary.MakeVector` 0.0 0.0 (* _position 700.0)) false false))
    (:`Finished`
      (`KismetSystemLibrary.Delay` 1.0)
      (`self.K2_DestroyActor`))))

(event `self.Attack_Collision.OnComponentBeginOverlap`
  (params (OverlappedComponent :type "PrimitiveComponent Object Reference") (OtherActor :type "Actor Object Reference") (OtherComp :type "PrimitiveComponent Object Reference") (OtherBodyIndex :type Integer) (bFromSweep :type Boolean) (SweepResult :type "HitResult Structure (by ref)"))
  (bind _asabyss_hand (cast `/Game/Blueprints/Abyss/Abyss_Hand` OtherActor))
  (`/Game/Blueprints/Abyss/Abyss_Hand.Take_Damage` _asabyss_hand (`KismetMathLibrary.Normal` (- (`self.K2_GetActorLocation` OtherActor) (`SceneComponent.K2_GetComponentLocation` (`self.Scale_Point1`)))) (`self.Damage_Type`) (`self.Damage`)))

(fn `UserConstructionScript`)