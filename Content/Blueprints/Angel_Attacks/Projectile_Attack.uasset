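; Projectile attack actor for the Angel's attacks, which moves a cube along Z and then removes itself.
; The Attack_Prj event plays a fire sound and runs a timeline that drives the cube's relative Z location.
; When the timeline finishes, the actor waits briefly and destroys itself.
; The event's scale multiplier input is not used, and the play rate is set on AttackTimeline.
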(event `Attack_Prj`
  (params (Scale_Multiplayer :type "Float (double-precision)"))
  (`TimelineComponent.SetPlayRate` (`self.Attack_Timeline`) 0.5)
  (`GameplayStatics.PlaySound2D` "/Game/Effects/Sound/AngelFirstFire.AngelFirstFire" 1.0 1.0 0.0 null null)
  (bind (_direction _scale _fade _position) (`Timeline|Attack_Timeline_Prj` :!via `PlayFromStart`)
    (:`Update`
      (`SceneComponent.K2_SetRelativeLocation` (`self.Cube`) (`KismetMathLibrary.MakeVector` 0.0 0.0 (* _position 100.0)) false false))
    (:`Finished`
      (`KismetSystemLibrary.Delay` 1.0)
      (`self.K2_DestroyActor`))))

(fn `UserConstructionScript`
  (`parent.UserConstructionScript`))