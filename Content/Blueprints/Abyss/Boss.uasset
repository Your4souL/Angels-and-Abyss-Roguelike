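; Abyss boss that repeatedly drops on a web to tear chunks out of the block island.
; HandAttack picks the farthest free block, excluding the last target, and a timeline stretches the web and lowers the boss facing field center.
; It darkens that block and its neighbors, attaches them after the obliterate timeline, then reverses the flight to lift, destroy and detach them before attacking again.
; Island-rotation flight logic is left unconnected.
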(event `self.Hand_Attack`
  (params (Start_Delay :type "Float (single-precision)") (FlyRate :type "Float (single-precision)"))
  (bind _target_block (`self.Target block`))
  (bind _returnvalue (`self.K2_GetActorLocation` _target_block))
  (`KismetSystemLibrary.Delay` Start_Delay)
  (`TimelineComponent.SetPlayRate` (`self.FlyTimeline`) (/ FlyRate 3.0))
  (set `self.Nearest_Dist` 0.0)
  (bind _returnvalue_2 (`GameplayStatics.GetActorOfClass` "/Game/Blueprints/BlockGridGenerator.BlockGridGenerator_C"))
  (bind _output_get (set `self.Island` _returnvalue_2))
  (for _array_element (`/Game/Blueprints/BlockGridGenerator.Blocks_Array` _output_get)
    (bind _returnvalue_3 (`self.GetDistanceTo` _array_element self))
    (if (and (not (`/Game/Blueprints/Block.Falling` _array_element)) (not (`/Game/Blueprints/Block.Occupied` _array_element)) (not (`/Game/Blueprints/Block.Z_covered` _array_element)) (> _returnvalue_3 (`self.Nearest_Dist`)) (!= (`self.Target block`) _array_element))
      (set `self.Nearest_Dist` _returnvalue_3)
      (bind _returnvalue_4 (`self.K2_GetActorLocation` _array_element))
      (bind _outhit (`KismetSystemLibrary.LineTraceSingle` (+ _returnvalue_4 (0.0 0.0 1000.0)) _returnvalue_4 "TraceTypeQuery1"))
      (bind _asblock (cast `/Game/Blueprints/Block` (`.HitActor` (`GameplayStatics.BreakHitResult` _outhit))))
      (set `self.Target block` _asblock)))
  (`/Engine/EditorBlueprintResources/StandardMacros.IsValid` _target_block
    (:`Is Valid`
      (`/Game/Blueprints/Block.Occupy` _target_block true)
      (set `self.End_Fly_Location` (+ _returnvalue (0.0 0.0 200.0)))
      (set `self.Start_Fly_Location` (+ _returnvalue (0.0 0.0 2500.0)))
      (bind (_direction _web _fly) (`Timeline|Web_Fly_Timeline` :!via `PlayFromStart` :!label _label)
        (:`Update`
          (`SceneComponent.SetRelativeScale3D` (`self.Web_Scene`) (`KismetMathLibrary.MakeVector` 0.01 0.01 (* _web 3.0)))
          (`self.K2_SetActorLocation` (`KismetMathLibrary.VLerp` (`self.Start_Fly_Location`) (`self.End_Fly_Location`) _fly))
          (bind _asroguelike_controller (cast `/Game/Blueprints/RoguelikeController` (`GameplayStatics.GetPlayerController` 0)))
          (bind (_returnvalue_roll _returnvalue_pitch _returnvalue_yaw) (`KismetMathLibrary.BreakRotator` (`KismetMathLibrary.FindLookAtRotation` (`self.K2_GetActorLocation`) (`/Game/Blueprints/RoguelikeController.Field_Center` _asroguelike_controller))))
          (`self.K2_SetActorRotation` (`KismetMathLibrary.MakeRotator` 0.0 0.0 _returnvalue_yaw)))
        (:`Finished`
          (switch `ETimelineDirection` _direction
            (:`Forward`
              (`self.Start_Obliterate`))
            (:`Backward`
              (for _array_element_2 (`self.Target_Blocks`)
                (`/Game/Blueprints/Block.On_Create` _array_element_2)
                (`/Game/Blueprints/Block.Fast_Obliterate` _array_element_2)
                (`self.K2_DetachFromActor` _array_element_2 "KeepWorld" "KeepWorld" "KeepWorld"))
              (`self.Hand_Attack` 0.0 5.0))))))))

(event `self.Obliterate_Block`
  (`Timeline|ObliterateTimeline` :!via `PlayFromStart`
    (:`Finished`
      (for _array_element (`self.Target_Blocks`)
        (`self.K2_AttachToActor` _array_element self "None" "KeepWorld" "KeepWorld" "KeepWorld" true)
        (`/Game/Blueprints/Block.Check_Near` _array_element true))
      (goto _label :!via `ReverseFromEnd`))))

(event `self.Break_Obliterate`)

(event `self.Take_Damage`
  (params (Direction :type "Vector Structure") (Damage_Source :type "/Game/Blueprints/Angel_Attacks/Damage_Type Enum" :default "NewEnumerator0") (Damage_Recieved :type Integer))
  (`parent.Take_Damage` Direction Damage_Source Damage_Recieved))

(event `Start_Obliterate`
  (bind _target_block (`self.Target block`))
  (set `self.Find_Angel_Distance` 0.0)
  (set `self.OnIsland` true)
  (`/Engine/EditorBlueprintResources/StandardMacros.IsValid` _target_block
    (:`Is Valid`
      (bind _blocks (`/Game/Blueprints/Block.Get_Near_Blocks` _target_block))
      (bind _output_get (set `self.Target_Blocks` _blocks))
      (for _array_element _output_get
        (`/Game/Blueprints/Block.Dark_Focus` _array_element false))
      (`/Game/Blueprints/Block.Dark_Focus` _target_block false)
      (`KismetArrayLibrary.Array_Add` (`self.Target_Blocks`) (`self.Target block`))
      (`self.Obliterate_Block`))))

(event `self.Custom_Action`
  (`self.Hand_Attack` 0.0 5.0))

(fn `UserConstructionScript`
  (`parent.UserConstructionScript`))