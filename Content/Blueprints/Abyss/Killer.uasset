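; Killer is a flying actor that hunts down fireplaces on the BlockGridGenerator island.
; HandAttack moves it to a WingedBase actor's height and caches the island.
; Its targeting loop, rerun when each flight finishes, flies toward a fireplace block, then highlights it, spins on a timeline and clears it.
; Without fireplaces it heads for the current custom target or island, picking a random AngelBase whenever it arrives.
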(event `self.Hand_Attack`
  (params (Start_Delay :type "Float (single-precision)") (FlyRate :type "Float (single-precision)"))
  (bind (_returnvalue_x _returnvalue_y) (`KismetMathLibrary.BreakVector` (`self.K2_GetActorLocation` self)))
  (`TimelineComponent.SetPlayRate` (`self.Fly_Timeline`) FlyRate)
  (bind _returnvalue (`GameplayStatics.GetActorOfClass` "/Game/Blueprints/WingedBase.WingedBase_C"))
  (bind _output_get (set `self.Custom_Target` _returnvalue))
  (bind (_returnvalue_x_2 _returnvalue_y_2 _returnvalue_z) (`KismetMathLibrary.BreakVector` (`self.K2_GetActorLocation` _output_get)))
  (`self.Custom_Fly` true 2.0 (`KismetMathLibrary.MakeVector` _returnvalue_x _returnvalue_y _returnvalue_z))
  (bind _returnvalue_2 (`GameplayStatics.GetActorOfClass` "/Game/Blueprints/BlockGridGenerator.BlockGridGenerator_C"))
  (set `self.Island` _returnvalue_2)
  (set `self.Custom_Target` null))

(event `self.Custom_Action`)

(event `Find_Fireplaces`
  (for _array_element (`/Game/Blueprints/BlockGridGenerator.Blocks_Array` (`self.Island`)) :!label _label
    (if (`/Game/Blueprints/Block.Have_Fireplace` _array_element)
      (set `self.Target block` _array_element)
      (`self.Break_Find_Fireplaces`))))

(event `Break_Find_Fireplaces`
  (goto _label :!via `Break`))

(event `Force_Find_Target`
  (bind _target_block (`self.Target block`))
  (bind _custom_target (`self.Custom_Target`))
  (bind _target_block_2 (`self.Target block`))
  (bind _lerping_start_pos (`self.Lerping_Start_Pos`))
  (bind (_returnvalue_roll _returnvalue_pitch _returnvalue_yaw) (`KismetMathLibrary.BreakRotator` (`self.K2_GetActorRotation` self)))
  (bind _returnvalue (`self.K2_GetActorLocation` (select `bool` (`KismetSystemLibrary.IsValid` _target_block) :`false` (select `bool` (`KismetSystemLibrary.IsValid` _custom_target) :`false` (`self.Island`) :`true` _custom_target :!type "Actor Object Reference") :`true` _target_block :!type "Actor Object Reference")))
  (set `self.Target block` null :!label _label_2)
  (`self.Find_Fireplaces`)
  (if (> (`KismetMathLibrary.Vector_Distance` (`self.K2_GetActorLocation` self) _returnvalue) 400.0)
    (`parent.Custom_Fly` false 0.2 (+ _returnvalue (0.0 0.0 300.0)))
    (else
      (`/Engine/EditorBlueprintResources/StandardMacros.IsValid` _target_block_2
        (:`Is Valid`
          (`/Game/Blueprints/Block.Dark_Focus` _target_block_2 true)
          (set `self.Lerping_Start_Pos` _returnvalue_yaw)
          (bind (_direction _alpha) (`Timeline|Destroy_Fireplace_Timeline` :!via `PlayFromStart`)
            (:`Update`
              (`self.K2_SetActorRelativeRotation` (`KismetMathLibrary.MakeRotator` 0.0 0.0 (`KismetMathLibrary.Lerp` _lerping_start_pos (+ _lerping_start_pos 720.0) _alpha))))
            (:`Finished`
              (switch `ETimelineDirection` _direction
                (:`Forward`
                  (`/Game/Blueprints/Block.Clear` (`self.Target block`))
                  (`self.Force_Find_Target`))))))
        (:`Is Not Valid`
          (bind _outactors (`GameplayStatics.GetAllActorsOfClass` "/Game/Blueprints/Buildable_Objects/AngelBase.AngelBase_C"))
          (bind _returnvalue_2 (`KismetArrayLibrary.Array_Length` _outactors))
          (if (> _returnvalue_2 0)
            (set `self.Custom_Target` (`|GetArrayItem` _outactors (`KismetMathLibrary.RandomIntegerInRange` 0 (- _returnvalue_2 1))))
            (`self.Force_Find_Target`)))))))

(event `self.Fly_Timeline__FinishedFunc`
  (goto _label_2))

(fn `UserConstructionScript`
  (`parent.UserConstructionScript`))