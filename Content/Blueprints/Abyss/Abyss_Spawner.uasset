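; Abyss wave spawner that launches timed, escalating enemy attacks from an arc around and below the world origin.
; Initiate loops via delay polling; tutorial mode scripts the first wave and gates progression on tips.
; StartWave spends a wave-scaled power budget on Hands, Salamanders or Killers, or spawns a Boss on wave three.
; Regular waves then rotate the attack arc and update the BlockGridGenerator preview; ControlClouds spins cloud layers.
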(event `Spawn_Unit`
  (params (Class :type "/Game/Blueprints/Abyss/Abyss_Hand Class Reference") (Delay_Order :type Integer))
  (bind _attack_angle (`self.Attack_Angle`))
  (bind _returnvalue (`|SpawnActorFromClass` Class (`KismetMathLibrary.MakeTransform` (+ (`KismetMathLibrary.GreaterGreater_VectorRotator` (4000.0 0.0 0.0) (`KismetMathLibrary.MakeRotator` 0.0 0.0 (+ (`KismetMathLibrary.RandomFloatInRange` 0.0 _attack_angle) (+ (/ _attack_angle -2.0) (`self.Attack_Angle_Offset`))))) (0.0 0.0 -2000.0))) "Undefined" "OverrideRootScale" null "NewEnumerator0" null))
  (`/Game/Blueprints/Abyss/Abyss_Hand.Hand_Attack` _returnvalue (* Delay_Order 1.0) 2.0)
  (`KismetArrayLibrary.Array_Add` (`self.Active Enemies`) _returnvalue)
  (set `/Game/Blueprints/Abyss/Abyss_Hand.Spawner` self _returnvalue))

(event `Initiate`
  (bind _controller_ref (`self.Controller_Ref`))
  (bind _controller_ref_2 (`self.Controller_Ref`))
  (bind _wave_number (`self.Wave_Number`))
  (`|ExecutionSequence`
    (:`then_0`
      (if (`/Game/Blueprints/RoguelikeController.Tutorial` (`self.Controller_Ref`))
        (`KismetSystemLibrary.PrintString` (`KismetStringLibrary.Concat_StrStr` "Wave " (`KismetStringLibrary.Conv_IntToString` _wave_number)) true true (struct :`R` 1.0 :`G` 0.033409 :`A` 1.0))
        (switch `int` _wave_number
          (:`Default`
            (`self.Start_Wave` (`self.Wave_Number`) :!label _label))
          (:`1`
            (for _index (range 5)
              (`self.Spawn_Unit` "/Game/Blueprints/Abyss/SmallSalamander.SmallSalamander_C" _index))
            (for _ (range 2)
              _)
            (set `/Game/Blueprints/RoguelikeController.Tutorial_Can_Next_Wave` false _controller_ref_2)))
        (else
          (goto _label))))
    (:`then_2`
      (bind _output_get (set `self.Next_Wave_Time` (+ (`GameplayStatics.GetTimeSeconds`) (`self.Waves_Delay`))))
      (if (< (`GameplayStatics.GetTimeSeconds`) _output_get) :!label _label_2
        (`KismetSystemLibrary.Delay` 0.016)
        (if (`/Game/Blueprints/RoguelikeController.Tutorial` _controller_ref_2)
          (if (and (== (`KismetArrayLibrary.Array_Length` (`self.Active Enemies`)) 0) (!= (`self.Wave_Number`) 0))
            (`KismetSystemLibrary.Delay` 0.5)
            (switch `int` (`self.Wave_Number`)
              (:`1`
                _)
              (:`2`
                _))
            (`/Game/Interface/Tutorial_Slides.Force_Next_Tip` (`/Game/Blueprints/RoguelikeController.Tutorial_Ref` (`self.Controller_Ref`)))
            (else
              (goto _label_2)))
          (else
            (goto _label_2)))
        (elif (`/Game/Blueprints/RoguelikeController.Tutorial` _controller_ref)
          (if (`/Game/Blueprints/RoguelikeController.Tutorial_Can_Next_Wave` _controller_ref)
            (`/Engine/EditorBlueprintResources/StandardMacros.IncrementInt` (`self.Wave_Number`) :!label _label_3
              (:`  `
                (`self.Initiate`))))
          (else
            (goto _label_3)))))))

(event `Wave_1`)

(event `Force_Next_Wave`
  (set `self.Next_Wave_Time` 0.0)
  (goto _label_2))

(event `Start_Wave`
  (params (Wave_Number :type Integer))
  (bind _attack_angle (`self.Attack_Angle`))
  (bind _output_get (set `self.Wave_Power` (* Wave_Number 3)))
  (if (== _output_get 9)
    (`self.Spawn_Unit` "/Game/Blueprints/Abyss/Boss.Boss_C")
    (else
      (if (> _output_get 0) :!label _label_4
        (`KismetSystemLibrary.Delay` 0.1)
        (`|ExecutionSequence`
          (:`then_0`
            (bind _returnvalue (`|SpawnActorFromClass` (select `bool` (and (>= (`self.Wave_Power`) 20) (< (`self.Number_Of_Killers`) 2)) :`false` (select `bool` (>= (`self.Wave_Power`) 5) :`false` "/Game/Blueprints/Abyss/Abyss_Hand.Abyss_Hand_C" :`true` "/Game/Blueprints/Abyss/SmallSalamander.SmallSalamander_C" :!type "Actor Class Reference") :`true` "/Game/Blueprints/Abyss/Killer.Killer_C") (`KismetMathLibrary.MakeTransform` (+ (`KismetMathLibrary.GreaterGreater_VectorRotator` (4000.0 0.0 0.0) (`KismetMathLibrary.MakeRotator` 0.0 0.0 (+ (`KismetMathLibrary.RandomFloatInRange` 0.0 _attack_angle) (+ (/ _attack_angle -2.0) (`self.Attack_Angle_Offset`))))) (0.0 0.0 -2000.0))) "Undefined" "OverrideRootScale" null null))
            (bind _asabyss_hand (cast `/Game/Blueprints/Abyss/Abyss_Hand` _returnvalue))
            (`/Game/Blueprints/Abyss/Abyss_Hand.Hand_Attack` _asabyss_hand 0.0 2.0)
            (set `self.Wave_Power` (- (`self.Wave_Power`) (select `/Game/Blueprints/Abyss/Abyss_Types` (`/Game/Blueprints/Abyss/Abyss_Hand.Type` _asabyss_hand) :`NewEnumerator0` 1 :`NewEnumerator1` 5 :`NewEnumerator2` 20)))
            (`KismetArrayLibrary.Array_Add` (`self.Active Enemies`) _asabyss_hand)
            (set `/Game/Blueprints/Abyss/Abyss_Hand.Spawner` self _asabyss_hand))
          (:`then_1`
            (goto _label_4)))
        (else
          (bind _output_get_2 (set `self.Attack_Angle_Offset` (+ (`self.Attack_Angle_Offset`) 90.0)))
          (bind _returnvalue_2 (`GameplayStatics.GetActorOfClass` "/Game/Blueprints/BlockGridGenerator.BlockGridGenerator_C"))
          (`/Game/Blueprints/BlockGridGenerator.Define_Attac_Preview` _returnvalue_2 _output_get_2))))))

(event `self.ReceiveBeginPlay`
  (bind _asroguelike_controller (cast `/Game/Blueprints/RoguelikeController` (`GameplayStatics.GetPlayerController` 0)))
  (set `self.Controller_Ref` _asroguelike_controller)
  (if (not (`/Game/Blueprints/RoguelikeController.Tutorial` _asroguelike_controller))
    (`self.Initiate`)))

(event `Control Clouds`
  (`SceneComponent.K2_AddLocalRotation` (`self.Cloud1`) (`KismetMathLibrary.MakeRotator` 0.0 0.0 (`KismetMathLibrary.RandomFloatInRange` 0.05 0.08)) false false)
  (`SceneComponent.K2_AddLocalRotation` (`self.Cloud2`) (`KismetMathLibrary.MakeRotator` 0.0 0.0 (`KismetMathLibrary.RandomFloatInRange` 0.2 0.3)) false false)
  (`SceneComponent.K2_AddLocalRotation` (`self.Cloud3`) (`KismetMathLibrary.MakeRotator` 0.0 0.0 (`KismetMathLibrary.RandomFloatInRange` -0.15 -0.05)) false false))

(fn `UserConstructionScript`)