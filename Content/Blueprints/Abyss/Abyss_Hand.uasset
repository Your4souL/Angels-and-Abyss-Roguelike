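; Abyss hand enemy that seizes blocks on the roguelike field and drags them down to obliterate them.
; It picks the nearest free Block, traces from above for the target, occupies it and flies over on a timeline, facing field center.
; A second timeline swings the hand, then attaches it to the sinking block.
; Damage reverses that timeline to release and retry, while death grants the player flame and removes it from the spawner.
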(event `Hand_Attack`
  (params (Start_Delay :type "Float (double-precision)") (FlyRate :type "Float (double-precision)"))
  (bind _target_block (`self.Target block`))
  (bind _custom_target (`self.Custom_Target`))
  (bind _target_block_2 (`self.Target block`))
  ;[1 1 1] Fly_Attack
  (`KismetSystemLibrary.Delay` Start_Delay)
  (`TimelineComponent.SetPlayRate` (`self.Fly_Timeline`) FlyRate)
  (set `self.Start_Fly_Location` (`self.K2_GetActorLocation`))
  (set `self.Nearest_Dist` 100000.0)
  (bind _outactors (`GameplayStatics.GetAllActorsOfClass` "/Game/Blueprints/Block.Block_C"))
  (for _array_element _outactors
    (bind _returnvalue (`self.GetDistanceTo` _array_element self))
    (if (and (not (`/Game/Blueprints/Block.Falling` _array_element)) (not (`/Game/Blueprints/Block.Occupied` _array_element)) (not (`/Game/Blueprints/Block.Z_covered` _array_element)) (< _returnvalue (`self.Nearest_Dist`)))
      (set `self.Nearest_Dist` _returnvalue)
      (bind _returnvalue_2 (`self.K2_GetActorLocation` _array_element))
      (bind _outhit (`KismetSystemLibrary.LineTraceSingle` (+ _returnvalue_2 (0.0 0.0 1000.0)) _returnvalue_2 "TraceTypeQuery1"))
      (bind _asblock (cast `/Game/Blueprints/Block` (`.HitActor` (`GameplayStatics.BreakHitResult` _outhit))))
      (set `self.Target block` _asblock)))
  (`/Engine/EditorBlueprintResources/StandardMacros.IsValid` _target_block_2
    (:`Is Valid`
      (`/Game/Blueprints/Block.Occupy` _target_block_2 true)
      (set `self.End_Fly_Location` (+ (`self.K2_GetActorLocation` _target_block_2) (0.0 0.0 200.0)))
      (bind (_direction _alpha) (`Timeline|Fly_Timeline` :!via `PlayFromStart` :!label _label)
        (:`Update`
          (`self.K2_SetActorLocation` (`KismetMathLibrary.VLerp` (`self.Start_Fly_Location`) (`self.End_Fly_Location`) _alpha))
          (if true
            (bind _asroguelike_controller (cast `/Game/Blueprints/RoguelikeController` (`GameplayStatics.GetPlayerController` 0)))
            (bind (_returnvalue_roll _returnvalue_pitch _returnvalue_yaw) (`KismetMathLibrary.BreakRotator` (`KismetMathLibrary.FindLookAtRotation` (`self.K2_GetActorLocation`) (`/Game/Blueprints/RoguelikeController.Field_Center` _asroguelike_controller))))
            (`self.K2_SetActorRotation` (`KismetMathLibrary.MakeRotator` 0.0 0.0 _returnvalue_yaw))))
        (:`Finished`
          (`/Engine/EditorBlueprintResources/StandardMacros.IsValid` _target_block
            (:`Is Valid`
              (`self.Obliterate_Block`)
              (`/Game/Blueprints/Block.Dark_Focus` _target_block false))
            (:`Is Not Valid`
              (`/Engine/EditorBlueprintResources/StandardMacros.IsValid` _custom_target
                (:`Is Valid`
                  (`KismetSystemLibrary.PrintString` (`KismetSystemLibrary.GetDisplayName` _custom_target) true true (struct :`R` 1.0 :`G` 0.153592 :`A` 1.0))
                  (`self.Custom_Action`))
                (:`Is Not Valid`
                  (`self.Hand_Attack` 0.0 1.0))))))))))

(event `Custom_Fly`
  (params (Face_To_Field_Center :type Boolean :default true) (Fly_Rate :type "Float (double-precision)") (Fly_Target :type "Vector Structure"))
  ;[1 1 1] Fly_Attack
  (`TimelineComponent.SetPlayRate` (`self.Fly_Timeline`) Fly_Rate)
  (set `self.End_Fly_Location` Fly_Target)
  (set `self.Start_Fly_Location` (`self.K2_GetActorLocation`))
  (set `self.Target block` null)
  (goto _label :!via `PlayFromStart`))

(event `Custom_Action`
  ;[1 1 1] Fly_Attack
)

(event `Obliterate_Block`
  (bind _target_block (`self.Target block`))
  (bind _target_block_2 (`self.Target block`))
  ;[1 1 1] Obliterate
  (`TimelineComponent.SetPlayRate` (`self.Obliterate_Timeline`) 1.0)
  (bind (_direction _alpha) (`Timeline|Obliterate_Timeline` :!via `PlayFromStart` :!label _label_2)
    (:`Update`
      (`/Engine/EditorBlueprintResources/StandardMacros.IsValid` _target_block_2
        (:`Is Valid`
          (`self.K2_SetActorLocation` (+ (`self.K2_GetActorLocation` _target_block_2) (0.0 0.0 200.0)))
          (`SceneComponent.K2_SetRelativeRotation` (`self.Rotating_Point`) (`KismetMathLibrary.RLerp` (struct :`Pitch` -80.0 :`Yaw` 180.0 :`Roll` 180.0) (struct :`Pitch` -20.0 :`Yaw` 180.0 :`Roll` 180.0) _alpha) false false))))
    (:`Finished`
      (switch `ETimelineDirection` _direction
        (:`Forward`
          (`self.K2_AttachToActor` _target_block "None" "KeepWorld" "KeepWorld" "KeepWorld")
          (`/Game/Blueprints/Block.On_Create` _target_block)
          (`/Game/Blueprints/Block.Obliterate` _target_block 0.7 -7000.0)
          (`KismetSystemLibrary.Delay` 3.0)
          (`KismetArrayLibrary.Array_RemoveItem` (`/Game/Blueprints/Abyss/Abyss_Spawner.Active Enemies` (`self.Spawner`)) self)
          (`self.K2_DestroyActor`))
        (:`Backward`
          (`self.Hand_Attack` 0.0 2.0))))))

(event `Break_Obliterate`
  (bind _target_block (`self.Target block`))
  ;[1 1 1] Obliterate
  (`TimelineComponent.SetPlayRate` (`self.Fly_Timeline`) 1.0)
  (`/Engine/EditorBlueprintResources/StandardMacros.IsValid` _target_block
    (:`Is Valid`
      (set `/Game/Blueprints/Block.Occupied` false _target_block)
      (goto _label_2 :!via `Reverse`))
    (:`Is Not Valid`
      (goto _label_2 :!via `Reverse`))))

(event `Show_Contur`
  (params (Show :type Boolean))
  (`PrimitiveComponent.SetRenderCustomDepth` (`self.Cube6`) Show)
  (`PrimitiveComponent.SetRenderCustomDepth` (`self.Cube`) Show)
  (`PrimitiveComponent.SetRenderCustomDepth` (`self.Cube4`) Show)
  (`PrimitiveComponent.SetRenderCustomDepth` (`self.Cube5`) Show)
  (`PrimitiveComponent.SetRenderCustomDepth` (`self.Cube1`) Show)
  (`PrimitiveComponent.SetRenderCustomDepth` (`self.Cube3`) Show)
  (`PrimitiveComponent.SetRenderCustomDepth` (`self.Cube2`) Show)
  (`PrimitiveComponent.SetRenderCustomDepth` (`self.Trail`) Show))

(event `Take_Damage`
  (params (Direction :type "Vector Structure") (Damage_Source :type "/Game/Blueprints/Angel_Attacks/Damage_Type Enum" :default "NewEnumerator0") (Damage_Recieved :type Integer))
  (bind _returnvalue (`self.K2_GetActorLocation`))
  ;[1 1 1] Damage from angels
  (`/Engine/EditorBlueprintResources/StandardMacros.DoOnce` false :!label _label_3
    (:`Completed`
      (`self.Break_Obliterate`)
      (`NiagaraFunctionLibrary.SpawnSystemAtLocation` "/Game/Effects/Abyss_Burst.Abyss_Burst" _returnvalue)
      (`NiagaraFunctionLibrary.SpawnSystemAtLocation` (select `/Game/Blueprints/Angel_Attacks/Damage_Type` Damage_Source :`NewEnumerator0` "/Game/Effects/Fireplace_Burst.Fireplace_Burst" :`NewEnumerator3` "/Game/Effects/Angel_Invoke.Angel_Invoke" :!type "NiagaraSystem Object Reference") _returnvalue)
      (bind _output_get (set `self.HP` (- (`self.HP`) Damage_Recieved)))
      (if (> _output_get 0)
        (`self.Reset_Take_Damage`)
        (else
          (bind _returnvalue_2 (`GameplayStatics.GetActorOfClass` "/Game/Blueprints/RoguelikeController.RoguelikeController_C"))
          (`/Game/Blueprints/RoguelikeController.Give_Flame` _returnvalue_2 3)
          (`KismetArrayLibrary.Array_RemoveItem` (`/Game/Blueprints/Abyss/Abyss_Spawner.Active Enemies` (`self.Spawner`)) self)
          (`self.K2_DestroyActor`))))))

(event `Reset_Take_Damage`
  ;[1 1 1] Damage from angels
  (`KismetSystemLibrary.Delay` 0.2)
  (goto _label_3 :!via `Reset`))

(fn `UserConstructionScript`)