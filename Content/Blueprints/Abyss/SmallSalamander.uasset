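; Small salamander unit that hops between field blocks, hunting angels or destroying the blocks it lands on.
; HandAttack claims the nearest free block and timeline-flies above it, facing the field center.
; It then seeks the nearest AngelBase, damaging it repeatedly in range or flying toward it via neighboring blocks.
; With no angels left, it obliterates and re-raises its block, then moves on; BreakObliterate cancels this.
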(event `self.Hand_Attack`
  (params (FlyRate :type "Float (single-precision)"))
  (bind _target_block (`self.Target block`))
  (`TimelineComponent.SetPlayRate` (`self.FlyTimeline`) FlyRate)
  (set `self.Start_Fly_Location` (`self.K2_GetActorLocation`))
  (set `self.Nearest_Dist` 100000.0)
  (bind _outactors (`GameplayStatics.GetAllActorsOfClass` "/Game/Blueprints/Block.Block_C"))
  (for _array_element _outactors
    (bind _returnvalue (`self.GetDistanceTo` _array_element self))
    (if (and (not (`/Game/Blueprints/Block.Falling` _array_element)) (not (`/Game/Blueprints/Block.Occupied` _array_element)) (not (`/Game/Blueprints/Block.Z_covered` _array_element)) (< _returnvalue (`self.Nearest_Dist`)) (!= _array_element (`self.Target block`)))
      (set `self.Nearest_Dist` _returnvalue)
      (bind _returnvalue_2 (`self.K2_GetActorLocation` _array_element))
      (bind _outhit (`KismetSystemLibrary.LineTraceSingle` (+ _returnvalue_2 (0.0 0.0 1000.0)) _returnvalue_2 "TraceTypeQuery1"))
      (bind _asblock (cast `/Game/Blueprints/Block` (`.HitActor` (`GameplayStatics.BreakHitResult` _outhit))))
      (set `self.Target block` _asblock)))
  (`/Engine/EditorBlueprintResources/StandardMacros.IsValid` _target_block
    (:`Is Valid`
      (`/Game/Blueprints/Block.Occupy` _target_block true)
      (set `self.End_Fly_Location` (+ (`self.K2_GetActorLocation` _target_block) (0.0 0.0 200.0)))
      (bind (_direction _alpha) (`Timeline|FlyTimeline` :!via `PlayFromStart`)
        (:`Update`
          (`self.K2_SetActorLocation` (`KismetMathLibrary.VLerp` (`self.Start_Fly_Location`) (`self.End_Fly_Location`) _alpha))
          (bind _asroguelike_controller (cast `/Game/Blueprints/RoguelikeController` (`GameplayStatics.GetPlayerController` 0)))
          (bind (_returnvalue_roll _returnvalue_pitch _returnvalue_yaw) (`KismetMathLibrary.BreakRotator` (`KismetMathLibrary.FindLookAtRotation` (`self.K2_GetActorLocation`) (`/Game/Blueprints/RoguelikeController.Field_Center` _asroguelike_controller))))
          (`self.K2_SetActorRotation` (`KismetMathLibrary.MakeRotator` 0.0 0.0 _returnvalue_yaw)))
        (:`Finished`
          (set `self.Find_Angel_Distance` 100000.0)
          (`self.Find Nearest Angel`))))))

(event `Find Nearest Angel`
  (bind _target_block (`self.Target block`))
  (bind _custom_target (`self.Custom_Target`))
  (bind _outactors (`GameplayStatics.GetAllActorsOfClass` "/Game/Blueprints/Buildable_Objects/AngelBase.AngelBase_C"))
  (if (> (`KismetArrayLibrary.Array_Length` _outactors) 0)
    (for _array_element _outactors
      (bind _returnvalue (`self.GetDistanceTo` _array_element self))
      (if (< _returnvalue (`self.Find_Angel_Distance`))
        (set `self.Find_Angel_Distance` _returnvalue)
        (set `self.Custom_Target` _array_element)))
    (if (> (`self.Find_Angel_Distance`) (`self.Attack_Distance`))
      (bind _result_block (`/Game/Blueprints/Block.Check_Near_Blocks_Distance_To_Target` (`self.Target block`) (`self.K2_GetActorLocation` _custom_target)))
      (`self.Custom_Fly` false 5.0 (+ (`self.K2_GetActorLocation` _result_block) (0.0 0.0 200.0)))
      (else
        (bind _asangel_base (cast `/Game/Blueprints/Buildable_Objects/AngelBase` _custom_target))
        (`/Game/Blueprints/Buildable_Objects/AngelBase.Take Damage` _asangel_base 1)
        (`KismetSystemLibrary.Delay` 1.0)
        (`self.Find Nearest Angel`)))
    (else
      (`/Engine/EditorBlueprintResources/StandardMacros.IsValid` _target_block
        (:`Is Valid`
          (`self.Obliterate_Block`)
          (`/Game/Blueprints/Block.Dark_Focus` _target_block))))))

(event `self.Obliterate_Block`
  (bind _target_block (`self.Target block`))
  (`Timeline|ObliterateTimeline` :!via `PlayFromStart` :!label _label
    (:`Finished`
      (`/Game/Blueprints/Block.On_Create` _target_block)
      (`/Game/Blueprints/Block.Rise` _target_block 0.7 -7000.0)
      (`self.Hand_Attack` 5.0))))

(event `self.Break_Obliterate`
  (bind _target_block (`self.Target block`))
  (`/Engine/EditorBlueprintResources/StandardMacros.IsValid` _target_block
    (:`Is Valid`
      (`/Game/Blueprints/Block.Cancel_Fall` _target_block)
      (set `/Game/Blueprints/Block.Occupied` false _target_block)
      (goto _label :!via `Stop`))
    (:`Is Not Valid`
      (goto _label :!via `Stop`))))

(event `self.Take_Damage`
  (params (Direction :type "Vector Structure") (Damage_Source :type "/Game/Blueprints/Angel_Attacks/Damage_Type Enum" :default "NewEnumerator0") (Damage_Recieved :type Integer))
  (`parent.Take_Damage` Direction Damage_Source Damage_Recieved))

(event `self.Custom_Action`
  (`self.Hand_Attack` 5.0))

(fn `UserConstructionScript`
  (`parent.UserConstructionScript`))