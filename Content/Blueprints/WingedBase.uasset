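; WingedBase is a winged, eyed base actor for a roguelike mode that grows through upgrades and drives an Omega Disk ring over the field.
; Upgrade raises capped WingPower and HP, revealing wing meshes, with extra eyes and ring parts at two milestones.
; Those milestones increase the ring's spin, which a once-gated timeline animates above FieldCenter with sparks.
; Tick bobs the skeletal mesh; Take_Damage is empty, leaving the game-over logic disconnected.
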(event `self.ReceiveBeginPlay`
  (set `self.WingMeshes` (`|MakeArray` (`self.Wing2`) (`self.Wing3`) (`self.Wing4`) (`self.Wing5`) (`self.Wing6`) (`self.Wing7`) (`self.Wing8`) (`self.Wing9`) (`self.Wing10`)))
  (set `/Game/Interface/InvisibleButton.Owner` self (cast `/Game/Interface/InvisibleButton` (`WidgetComponent.GetWidget` (`self.Button`)) :!pure true))
  (set `self.Wing_Power` (* 10 (`self.Wing_Power_Multiplyer`)))
  (`KismetSystemLibrary.Delay` 0.0)
  (bind _asroguelike_controller (cast `/Game/Blueprints/RoguelikeController` (`GameplayStatics.GetPlayerController` 0)))
  (`SceneComponent.K2_SetWorldLocation` (`self.Ring`) (+ (`/Game/Blueprints/RoguelikeController.Field_Center` _asroguelike_controller) (0.0 0.0 3000.0)) false false))

(event `Show_Countur`
  (params (Show :type Boolean))
  (`PrimitiveComponent.SetRenderCustomDepth` (`self.Wing1`) Show))

(event `self.ReceiveTick`
  (params (DeltaSeconds :type "Float (single-precision)"))
  (bind _relativescale3d_x (`KismetMathLibrary.BreakVector` (`SceneComponent.RelativeScale3D` (`self.Wing1`))))
  (`SceneComponent.K2_SetRelativeLocation` (`self.SkeletalMesh1`) (`KismetMathLibrary.MakeVector` 0.0 0.0 (- (* (`KismetMathLibrary.Sin` (* (`GameplayStatics.GetTimeSeconds`) 3.0)) (* _relativescale3d_x 5.0)) -40.0)) false false))

(event `Upgrade`
  (bind _wing_power_multiplyer (`self.Wing_Power_Multiplyer`))
  (bind _returnvalue (* 10 _wing_power_multiplyer))
  (bind _output_get (set `self.Wing_Power` (`KismetMathLibrary.FMin` (+ (`self.Wing_Power`) _returnvalue) (* 100 _wing_power_multiplyer))))
  (bind _returnvalue_2 (`KismetMathLibrary.FTrunc` (/ (- _output_get (* 20 _wing_power_multiplyer)) _returnvalue)))
  (`SceneComponent.SetHiddenInGame` (`|GetArrayItem` (`self.WingMeshes`) _returnvalue_2) false false)
  (set `self.HP` (`KismetMathLibrary.Min` (+ (`self.HP`) 1) 10))
  (switch `int` _returnvalue_2
    (:`3`
      (`SceneComponent.SetHiddenInGame` (`self.SeparateEyeOther2`) false false)
      (`SceneComponent.SetVisibility` (`self.SeparateEyeOther6`) true false)
      (`SceneComponent.SetVisibility` (`self.SeparateEyeOther5`) true false)
      (`SceneComponent.SetVisibility` (`self.SeparateEyeOther4`) true false)
      (`SceneComponent.SetVisibility` (`self.SeparateEyeOther3`) true false)
      (`SceneComponent.SetVisibility` (`self.Ring2`) true false)
      (`SceneComponent.SetVisibility` (`self.RingWing3`) true false)
      (`SceneComponent.SetVisibility` (`self.RingWing4`) true false)
      (set `self.RIng_Rotattion_Summ` -3240.0))
    (:`7`
      (`SceneComponent.SetHiddenInGame` (`self.SeparateEyeOther1`) false false)
      (`SceneComponent.SetVisibility` (`self.RingWing5`) true false)
      (`SceneComponent.SetVisibility` (`self.RingWing6`) true false)
      (`SceneComponent.SetVisibility` (`self.RingWing7`) true false)
      (`SceneComponent.SetVisibility` (`self.RingWing8`) true false)
      (`SceneComponent.SetVisibility` (`self.SeparateEyeOther7`) true false)
      (`SceneComponent.SetVisibility` (`self.SeparateEyeOther8`) true false)
      (`SceneComponent.SetVisibility` (`self.SeparateEyeOther9`) true false)
      (`SceneComponent.SetVisibility` (`self.SeparateEyeOther10`) true false)
      (set `self.RIng_Rotattion_Summ` -4320.0))))

(event `Call_Omega_Disk`
  (`TimelineComponent.SetPlayRate` (`self.Omega_Disk_Timeline`) (/ -4320.0 (`self.RIng_Rotattion_Summ`)))
  (`/Engine/EditorBlueprintResources/StandardMacros.DoOnce` false :!label _label
    (:`Completed`
      (bind (_direction _poition_alpha _rotation) (`Timeline|Omega_Disk_Timeline` :!via `PlayFromStart`)
        (:`Update`
          (`SceneComponent.K2_SetWorldLocationAndRotation` (`self.Ring`) (+ (`/Game/Blueprints/RoguelikeController.Field_Center` (cast `/Game/Blueprints/RoguelikeController` (`GameplayStatics.GetPlayerController` 0) :!pure true)) (`KismetMathLibrary.VLerp` (0.0 0.0 1500.0) (0.0 0.0 2500.0) _poition_alpha)) (`KismetMathLibrary.MakeRotator` 0.0 90.0 (* _rotation (`self.RIng_Rotattion_Summ`))) false false)
          (`ActorComponent.SetActive` (`self.Sparks`) true false))
        (:`Finished`
          (goto _label :!via `Reset`))))))

(event `Take_Damage`
  (params (Damage :type Integer)))

(fn `UserConstructionScript`)