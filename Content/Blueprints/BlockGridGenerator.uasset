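; Block grid generator that builds the roguelike's layered island on BeginPlay or Recreate_Level and places the player's WingedBase.
; It spawns a circular grid of randomly rotated blocks, erodes it by distance-weighted random falls and neighbour checks, then stacks raised layers around two peaks.
; Shuffled passes pick open blocks for fireplaces and the base, which is handed to RoguelikeController.
; It also loops a camera shake, counts island mass and has helpers for direction-click targeting.
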(event `Recreate_Level`
  (bind _blocks_array (`self.Blocks_Array`))
  (bind _blocks_array_2 (`self.Blocks_Array`))
  (bind _size (`self.Size`))
  (bind _blockspacing (`self.BlockSpacing`))
  (bind _size_2 (`self.Size`))
  (bind _blocks_array_3 (`self.Blocks_Array`))
  (bind _pike1 (`self.Pike1`))
  (bind _blockspacing_2 (`self.BlockSpacing`))
  (bind _returnvalue (/ (`self.Size`) 2))
  (bind _returnvalue_2 (/ (`self.Size`) 2))
  ;[1 1 1] Spawn blocks
  (for _array_element _blocks_array
    (`self.K2_DestroyActor` _array_element))
  (`KismetArrayLibrary.Array_Clear` _blocks_array)
  (for _index (range (* _size _size)) :!label _label
    (bind _returnvalue_3 (mod _index _size_2))
    (bind _returnvalue_4 (- _returnvalue _returnvalue_3))
    (bind _returnvalue_5 (/ _index _size_2))
    (bind _returnvalue_6 (- _returnvalue _returnvalue_5))
    (if (< (+ (* _returnvalue_4 _returnvalue_4) (* _returnvalue_6 _returnvalue_6)) 40)
      (bind _returnvalue_7 (`|SpawnActorFromClass` "/Game/Blueprints/Block.Block_C" (`KismetMathLibrary.MakeTransform` (+ (`KismetMathLibrary.MakeVector` (* _returnvalue_3 _blockspacing_2) (* _returnvalue_5 _blockspacing_2) _blockspacing_2) (`self.K2_GetActorLocation`)) (struct) (2.0 2.0 2.0)) "AlwaysSpawn" "OverrideRootScale" null self _returnvalue_3 _returnvalue_5 0 null)) ; Spawn a  block
      (`KismetArrayLibrary.Array_Add` (`self.Blocks_Array`) _returnvalue_7)
      (`/Game/Blueprints/Block.On_Create` _returnvalue_7)
      (bind _output_get (set `/Game/Blueprints/Block.Fall_Rotator` (`KismetMathLibrary.MakeRotator` (* (`KismetMathLibrary.RandomIntegerInRange` 0 3) 90.0) (* (`KismetMathLibrary.RandomIntegerInRange` 0 3) 90.0) (* (`KismetMathLibrary.RandomIntegerInRange` 0 3) 90.0)) _returnvalue_7))
      (`SceneComponent.K2_SetWorldRotation` (`/Game/Blueprints/Block.BlockMesh` _returnvalue_7) _output_get false false)
      (`SceneComponent.K2_SetWorldRotation` :`self` (`/Game/Blueprints/Block.Fireplace_Scene` _returnvalue_7))))
  ;[1 1 1] Basic Distruction
  (for _array_element_2 (`self.Blocks_Array`)
    (bind _returnvalue_8 (- _returnvalue_2 (`/Game/Blueprints/Block.X_pos` _array_element_2)))
    (bind _returnvalue_9 (- _returnvalue_2 (`/Game/Blueprints/Block.Y_pos` _array_element_2)))
    (bind _output_get_2 (set `/Game/Blueprints/Block.Destroy_Chance` (* (+ (/ (`KismetMathLibrary.Conv_IntToDouble` (* _returnvalue_8 _returnvalue_8)) _blockspacing) (/ (`KismetMathLibrary.Conv_IntToDouble` (* _returnvalue_9 _returnvalue_9)) _blockspacing)) (`self.Decay_Factor`)) _array_element_2))
    (if (> _output_get_2 (`KismetMathLibrary.RandomFloatInRange` (`self.Save_Offset`) (`self.Decay_Offset`)))
      (`/Game/Blueprints/Block.Fall` _array_element_2)))
  ;[1 1 1] Advanced Distruction
  (for _array_element_3 (`self.Blocks_Array`)
    (if (not (`/Game/Blueprints/Block.Falling` _array_element_3))
      (`/Game/Blueprints/Block.Check_Near` _array_element_3 false)))
  (for _array_element_4 (`self.Blocks_Array`)
    (`/Game/Blueprints/Block.NearFall` _array_element_4 7))
  ;[1 1 1] Generate new layers of blocks
  (`self.Generate layer` _pike1 5 1)
  (`self.Generate layer` _pike1 6 2)
  (`self.Generate layer` (`self.Pike2`) 5 1)
  ;[1 1 1] Setup fireplaces
  (`KismetArrayLibrary.Array_Shuffle` _blocks_array_3)
  (for _array_element_5 _blocks_array_3 :!label _label_2
    (if (> (`self.Fireplaces_Number`) 0)
      (if (and (not (`/Game/Blueprints/Block.Z_covered` _array_element_5)) (not (`/Game/Blueprints/Block.Falling` _array_element_5)) (not (`/Game/Blueprints/Block.Occupied` _array_element_5)) (== (`/Game/Blueprints/Block.Z_pos` _array_element_5) 1))
        (`/Game/Blueprints/Block.Enable_Fireplce` _array_element_5)
        (`/Engine/EditorBlueprintResources/StandardMacros.DecrementInt` (`self.Fireplaces_Number`)))
      (else
        (`self.Break_Fireplaces_Setting`))))
  ;[1 1 1] Setup Base
  (`KismetArrayLibrary.Array_Shuffle` _blocks_array_2)
  (for _array_element_6 _blocks_array_2 :!label _label_3
    (if (and (== (`/Game/Blueprints/Block.Z_pos` _array_element_6) 0) (not (`/Game/Blueprints/Block.Z_covered` _array_element_6)) (not (`/Game/Blueprints/Block.Occupied` _array_element_6)))
      (bind _output_get_3 (set `self.Emphemering_Block` _array_element_6))
      (set `/Game/Blueprints/Block.Occupied` true _output_get_3)
      (`PrimitiveComponent.SetMaterial` (`/Game/Blueprints/Block.BlockMesh` _output_get_3) 0 "/Game/Meshes/_Materials/Cubes/BlueCube.BlueCube")
      (`self.Break_Base_Finding`)))
  (bind _returnvalue_10 (`|SpawnActorFromClass` "/Game/Blueprints/WingedBase.WingedBase_C" (`KismetMathLibrary.MakeTransform` (+ (`self.K2_GetActorLocation` (`self.Emphemering_Block`)) (0.0 0.0 100.0)) (struct) (5.0 5.0 5.0)) "Undefined" "OverrideRootScale" null null))
  (bind _asroguelike_controller (cast `/Game/Blueprints/RoguelikeController` (`GameplayStatics.GetPlayerController` 0)))
  (set `/Game/Blueprints/RoguelikeController.Base_to_Upgrade` _returnvalue_10 _asroguelike_controller))

(event `self.ReceiveBeginPlay`
  ;[1 1 1] Spawn blocks
  (`|ExecutionSequence`
    (:`then_0`
      (goto _label))
    (:`then_2`
      (`GameplayStatics.PlayWorldCameraShake` "/Game/Effects/Falling_Camera_Shake.Falling_Camera_Shake_C" (`SceneComponent.K2_GetComponentLocation` (`self.Plain`)) 0.0 100000.0 :!label _label_4)
      (`KismetSystemLibrary.Delay` 60.0)
      (goto _label_4))))

(event `Generate layer`
  (params (PikePos :type "IntPoint Structure") (NearBlocksFactor :type Integer :default 5) (Z_pos :type Integer))
  (bind (_x _y) (break `IntPoint` PikePos))
  (bind _returnvalue (/ (* (`self.Size`) (`self.BlockSpacing`)) (`self.Relief_Decay_Factor`)))
  ;[1 1 1] Generate new layers of blocks
  (for _array_element (`self.Blocks_Array`)
    (`/Game/Blueprints/Block.Check_Near` _array_element false)
    (bind _returnvalue_2 (- _x (`/Game/Blueprints/Block.X_pos` _array_element)))
    (bind _returnvalue_3 (- _y (`/Game/Blueprints/Block.Y_pos` _array_element)))
    (if (and (> 0.25 (+ (/ (`KismetMathLibrary.Conv_IntToDouble` (* _returnvalue_2 _returnvalue_2)) _returnvalue) (/ (`KismetMathLibrary.Conv_IntToDouble` (* _returnvalue_3 _returnvalue_3)) _returnvalue))) (not (`/Game/Blueprints/Block.Falling` _array_element)) (> (`/Game/Blueprints/Block.Near_Blocks_Number` _array_element) NearBlocksFactor) (== (`/Game/Blueprints/Block.Z_pos` _array_element) (- Z_pos 1)))
      (set `/Game/Blueprints/Block.Z_covered` true _array_element)
      (bind _returnvalue_4 (`|SpawnActorFromClass` "/Game/Blueprints/Block.Block_C" (`KismetMathLibrary.MakeTransform` (+ (`self.K2_GetActorLocation` _array_element) (`KismetMathLibrary.MakeVector` 0.0 0.0 (`self.BlockSpacing`))) (struct) (2.0 2.0 2.0)) "AlwaysSpawn" "OverrideRootScale" null self (`/Game/Blueprints/Block.X_pos` _array_element) (`/Game/Blueprints/Block.Y_pos` _array_element) Z_pos null)) ; Spawn a  block
      (`KismetArrayLibrary.Array_Add` (`self.Blocks_Array`) _returnvalue_4)
      (`/Game/Blueprints/Block.On_Create` _returnvalue_4)
      (bind _output_get (set `/Game/Blueprints/Block.Fall_Rotator` (`KismetMathLibrary.MakeRotator` (* (`KismetMathLibrary.RandomIntegerInRange` 0 3) 90.0) (* (`KismetMathLibrary.RandomIntegerInRange` 0 3) 90.0) (* (`KismetMathLibrary.RandomIntegerInRange` 0 3) 90.0)) _returnvalue_4))
      (`SceneComponent.K2_SetWorldRotation` (`/Game/Blueprints/Block.BlockMesh` _returnvalue_4) _output_get false false)
      (`SceneComponent.K2_SetWorldRotation` :`self` (`/Game/Blueprints/Block.Fireplace_Scene` _returnvalue_4)))))

(event `Break_Fireplaces_Setting`
  ;[1 1 1] Setup fireplaces
  (goto _label_2 :!via `Break`))

(event `After_Direction_Click`
  (params (Exception_Block :type "/Game/Blueprints/Block Object Reference"))
  (for _array_element (`self.Blocks_Array`)
    (if (!= _array_element Exception_Block)
      (`/Game/Blueprints/Block.Unavilible_For_Direction_Click` _array_element))))

(event `Break_Base_Finding`
  ;[1 1 1] Setup Base
  (goto _label_3 :!via `Break`))

(event `Define_Attac_Previw`
  (params (Angle :type "Float (double-precision)"))
  (`SceneComponent.K2_SetRelativeRotation` (`self.Attack_Preview`) (`KismetMathLibrary.MakeRotator` 0.0 0.0 Angle) false false))

(event `BreakGrassGrowth`
  (bind _blocks_array (`self.Blocks_Array`))
  ;[1 1 1] Grow Grass
  (for _array_element (`self.Blocks_Array`) :!via `Break`
    (if (> (`self.Grass_Number`) 0)
      (bind _z_pos (`/Game/Blueprints/Block.Z_pos` _array_element))
      (if (and (not (`/Game/Blueprints/Block.Z_covered` _array_element)) (not (`/Game/Blueprints/Block.Falling` _array_element)) (not (`/Game/Blueprints/Block.Occupied` _array_element)) (> _z_pos 0) (< _z_pos 2))
        (`/Game/Blueprints/Block.GrowGrass` _array_element)
        (`/Engine/EditorBlueprintResources/StandardMacros.DecrementInt` (`self.Grass_Number`)))
      (else
        (`self.BreakGrassGrowth`))))
  ;[1 1 1] Add_Water
  (`KismetArrayLibrary.Array_Shuffle` _blocks_array)
  (for _array_element_2 _blocks_array :!label _label_5
    (if (> (`self.Water_Number`) 0)
      (if (and (not (`/Game/Blueprints/Block.Z_covered` _array_element_2)) (not (`/Game/Blueprints/Block.Falling` _array_element_2)) (not (`/Game/Blueprints/Block.Occupied` _array_element_2)) (< (`/Game/Blueprints/Block.Z_pos` _array_element_2) 1))
        (`/Game/Blueprints/Block.Add_Water` _array_element_2)
        (`/Engine/EditorBlueprintResources/StandardMacros.DecrementInt` (`self.Water_Number`)))
      (else
        (`self.Break_Adding_Water`)))))

(event `Break_Adding_Water`
  ;[1 1 1] Add_Water
  (goto _label_5 :!via `Break`))

(fn `Get_Island_Mass`
  (returns (SummMass :type "Float (double-precision)"))
  (locals (Mass :type "Float (double-precision)"))
  (set `local.Mass` 0.0)
  (for _array_element (`self.Blocks_Array`)
    (if (`/Game/Blueprints/Block.Have_Mass` _array_element)
      (`/Engine/EditorBlueprintResources/StandardMacros.IncrementFloat` (`local.Mass`))))
  (return (`local.Mass`)))

(fn `UserConstructionScript`
  (bind _plain (`self.Plain`))
  (bind _returnvalue (* (`self.Size`) 1.5))
  (bind _returnvalue_2 (/ (* (* (+ (`self.Size`) 1) -1) (`self.BlockSpacing`)) 2.0))
  (`SceneComponent.K2_AddLocalOffset` _plain (`KismetMathLibrary.MakeVector` _returnvalue_2 _returnvalue_2) false false)
  (`SceneComponent.SetRelativeScale3D` _plain (`KismetMathLibrary.MakeVector` _returnvalue _returnvalue 1.0)))