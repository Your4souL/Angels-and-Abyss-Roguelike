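; Legioneer is a buildable, winged angel turret that shoots projectiles at actors tagged "Abyss."
; Initiate drives a sine-based wing wobble, targeting of the nearest enemy within a range band, and DoOnce-gated firing on a cooldown.
; Shots spawn at the eye light with bonus damage and a distance-scaled attack parameter.
; Upgrades use a FlipFlop to reveal extra wing pairs and set attack interval and aim range.
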(event `self.OnInvoke`
  (`parent.OnInvoke`)
  (`GameplayStatics.PlaySound2D` "/Game/Effects/Sound/AngelFirstSummon.AngelFirstSummon" 1.0 1.0 0.33 null null)
  ;[1 1 1] Invoke Animations
  (`KismetSystemLibrary.Delay` 0.6)
  (`SkeletalMeshComponent.PlayAnimation` (`self.Winglvl1_2`) "/Game/Meshes/Singular_Wing/SeparateWingAnim2_Anim.SeparateWingAnim2_Anim" true)
  (`SkeletalMeshComponent.PlayAnimation` (`self.Winglvl1_1`) "/Game/Meshes/Singular_Wing/SeparateWingAnim2_Anim.SeparateWingAnim2_Anim" true)
  (`SkeletalMeshComponent.PlayAnimation` (`self.Winglvl3_2`) "/Game/Meshes/Singular_Wing/WingLowAnim.WingLowAnim" true)
  (`SkeletalMeshComponent.PlayAnimation` (`self.Winglvl2_1`) "/Game/Meshes/Singular_Wing/WingLowAnim.WingLowAnim" true)
  (`SkeletalMeshComponent.PlayAnimation` (`self.Winglvl2_2`) "/Game/Meshes/Singular_Wing/WingLowAnim.WingLowAnim" true)
  (`SkeletalMeshComponent.PlayAnimation` (`self.Winglvl3_1`) "/Game/Meshes/Singular_Wing/WingLowAnim.WingLowAnim" true))

(event `self.OnExile`
  (params (Delay :type Boolean))
  (`parent.OnExile` Delay))

(event `Custom wing movement`
  (bind _winglvl1_1 (`self.Winglvl1_1`))
  (bind _returnvalue (`KismetMathLibrary.DegSin` (* -360 (/ (`SkeletalMeshComponent.GetPosition` _winglvl1_1) 2.58))))
  ;[1 1 1] Custom wing movement
  (`SceneComponent.K2_SetRelativeRotation` _winglvl1_1 (`KismetMathLibrary.MakeRotator` (+ -90.0 (* 10 _returnvalue)) 0.0 -10.0) false false)
  (`SceneComponent.K2_SetRelativeRotation` (`self.Winglvl1_2`) (`KismetMathLibrary.MakeRotator` (+ -90.0 (* -10 _returnvalue)) 0.0 10.0) false false))

(event `self.Initiate`
  ;[1 1 1] initiate cycle
  (`self.Custom wing movement`)
  (`self.Aim`)
  (`self.TryShoot`)
  (`parent.Initiate`))

(event `self.Upgrade`
  (bind _winglvl2_2 (`self.Winglvl2_2`))
  (`parent.Upgrade`)
  (`/Engine/EditorBlueprintResources/StandardMacros.FlipFlop`
    (:`A`
      (`SceneComponent.SetHiddenInGame` (`self.Winglvl3_2`) false false)
      (`SceneComponent.SetHiddenInGame` (`self.Winglvl3_1`) false false)
      (`PrimitiveComponent.SetCollisionEnabled` (`self.Winglvl3_1`) "QueryAndPhysics")
      (`PrimitiveComponent.SetCollisionEnabled` (`self.Winglvl3_2`) "QueryAndPhysics")
      (set `self.Attack_Interval` 2.0)
      (set `self.Aim_Distance` 800.0))
    (:`B`
      (`SceneComponent.SetHiddenInGame` _winglvl2_2 false false)
      (`SceneComponent.SetHiddenInGame` (`self.Winglvl2_1`) false false)
      (`PrimitiveComponent.SetCollisionEnabled` _winglvl2_2 "QueryAndPhysics")
      (`PrimitiveComponent.SetCollisionEnabled` (`self.Winglvl2_1`) "QueryAndPhysics")
      (set `self.Attack_Interval` 1.0)
      (set `self.Aim_Distance` 1000.0))))

(event `Aim`
  (bind (_returnvalue_roll _returnvalue_pitch _returnvalue_yaw) (`KismetMathLibrary.BreakRotator` (`KismetMathLibrary.FindLookAtRotation` (`SceneComponent.K2_GetComponentLocation` (`self.Ray1_Eye_Light`)) (`self.Hit_Location`))))
  ;[1 1 1] Aim
  (set `self.Distance_tmp` (`self.Aim_Distance`))
  (bind _outactors (`GameplayStatics.GetAllActorsWithTag` "Abyss"))
  (if (> (`KismetArrayLibrary.Array_Length` _outactors) 0)
    (for _array_element _outactors
      (bind _returnvalue (`self.GetDistanceTo` _array_element self))
      (if (and (< _returnvalue (`self.Distance_tmp`)) (> _returnvalue 100.0))
        (set `self.Hit_Location` (+ (`self.K2_GetActorLocation` _array_element) (0.0 0.0 50.0)))
        (set `self.Distance_tmp` _returnvalue)))
    (set `self.Shoot_Angle` (`KismetMathLibrary.MakeRotator` _returnvalue_roll _returnvalue_pitch _returnvalue_yaw))))

(event `Shoot`
  (params (Dir :type "Rotator Structure"))
  ;[1 1 1] Shooting
  (bind _returnvalue (`|SpawnActorFromClass` "/Game/Blueprints/Angel_Attacks/Projectile_Attack.Projectile_Attack_C" (`KismetMathLibrary.MakeTransform` (+ (`SceneComponent.K2_GetComponentLocation` (`self.Ray1_Eye_Light`)) (`KismetMathLibrary.GreaterGreater_VectorRotator` (-30.0 0.0 0.0) Dir)) Dir (2.0 2.0 2.0)) "Undefined" "OverrideRootScale" null (+ (`self.Damage`) (`self.Bonus_Damage`)) "NewEnumerator3" null))
  (`/Game/Blueprints/Angel_Attacks/Projectile_Attack.Attack_Prj` _returnvalue (/ (`self.Distance_tmp`) 40.0))
  (set `self.Hit_Location` (0.0 0.0 0.0)))

(event `TryShoot`
  ;[1 1 1] Shooting
  ;;[1 1 1] Trying
  (if (!= (`KismetMathLibrary.VSize` (`self.Hit_Location`)) 0.0)
    (`KismetSystemLibrary.Delay` 0.2)
    (`/Engine/EditorBlueprintResources/StandardMacros.DoOnce` false :!label _label
      (:`Completed`
        (`self.Shoot` (`self.Shoot_Angle`))
        (`KismetSystemLibrary.Delay` (`self.Attack_Interval`))
        (goto _label :!via `Reset`)))))

(fn `UserConstructionScript`
  (`parent.UserConstructionScript`))