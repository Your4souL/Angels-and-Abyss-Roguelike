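; Buildable laser turret that fires Ray_Attack projectiles when Abyss_Hand actors enter its capsule, building on parent invoke, exile and upgrade logic.
; Invoking starts looping wing animations after a short delay; Initiate runs Aim, then TryShoot.
; Aim takes the eye sphere's current yaw rather than the target's position.
; Shots are throttled by a DoOnce reset after AttackInterval, carry base plus bonus damage, and spin the sphere in a random direction.
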(event `self.ReceiveBeginPlay`
  (set `self.Invoke_Z_Scale` 100 :!label _label)
  (`parent.OnInvoke`)
  ;[1 1 1] Invoke Animations
  (`KismetSystemLibrary.Delay` 0.6)
  (`SkeletalMeshComponent.PlayAnimation` (`self.Winglvl1_2`) "/Game/Meshes/Singular_Wing/WingLowAnim.WingLowAnim" true)
  (`SkeletalMeshComponent.PlayAnimation` (`self.Winglvl1_1`) "/Game/Meshes/Singular_Wing/WingLowAnim.WingLowAnim" true)
  (`SkeletalMeshComponent.PlayAnimation` (`self.Winglvl1_3`) "/Game/Meshes/Singular_Wing/SeparateWingAnim2_Anim.SeparateWingAnim2_Anim" true)
  (`SkeletalMeshComponent.PlayAnimation` (`self.Winglvl1_4`) "/Game/Meshes/Singular_Wing/SeparateWingAnim2_Anim.SeparateWingAnim2_Anim" true))

(event `self.OnInvoke`
  (goto _label))

(event `self.OnExile`
  (params (Delay :type Boolean))
  (`parent.OnExile` false))

(event `Custom wing movement`
  ;[1 1 1] Custom wing movement
)

(event `self.Initiate`
  ;[1 1 1] initiate cycle
  (bind _output_get (set `self.Floating_Offset` 5.0))
  (set `self.Floating_Scale` (`KismetMathLibrary.FTrunc` _output_get))
  (`self.Custom wing movement`)
  (`self.Aim`)
  (`self.TryShoot`)
  (`parent.Initiate`))

(event `self.Upgrade`
  (`parent.Upgrade`)
  (`/Engine/EditorBlueprintResources/StandardMacros.FlipFlop`))

(event `Aim`
  (bind _ray_1_sphere (`self.Ray_1_Sphere`))
  (bind (_returnvalue_roll _returnvalue_pitch _returnvalue_yaw) (`KismetMathLibrary.BreakRotator` (`SceneComponent.K2_GetComponentRotation` _ray_1_sphere)))
  ;[1 1 1] Aim
  (if (> (`KismetArrayLibrary.Array_Length` (`PrimitiveComponent.GetOverlappingActors` (`self.Capsule`) "/Game/Blueprints/Abyss/Abyss_Hand.Abyss_Hand_C")) 0)
    (set `self.Hit_Location` (+ (`KismetMathLibrary.GreaterGreater_VectorRotator` (1000.0 0.0 0.0) (`KismetMathLibrary.MakeRotator` 0.0 0.0 _returnvalue_yaw)) (`SceneComponent.K2_GetComponentLocation` _ray_1_sphere)))
    (set `self.Shoot_Angle` (`KismetMathLibrary.MakeRotator` 0.0 0.0 _returnvalue_yaw))))

(event `Shoot`
  (params (Dir :type "Rotator Structure"))
  ;[1 1 1] Shooting
  (`|ExecutionSequence`
    (:`then_0`
      (bind _returnvalue (`|SpawnActorFromClass` "/Game/Blueprints/Angel_Attacks/Ray_Attack.Ray_Attack_C" (`KismetMathLibrary.MakeTransform` (+ (`SceneComponent.K2_GetComponentLocation` (`self.Ray1_Eye_Light`)) (`KismetMathLibrary.GreaterGreater_VectorRotator` (-30.0 0.0 0.0) Dir)) Dir) "Undefined" "OverrideRootScale" null (+ (`self.Damage`) (`self.Bonus_Damage`)) "NewEnumerator3" null))
      (`/Game/Blueprints/Angel_Attacks/Ray_Attack.Attack` _returnvalue 20.0)
      (set `self.Hit_Location` (0.0 0.0 0.0)))
    (:`then_1`
      (set `self.Attack_Rotate_Dir` (select `bool` (`KismetMathLibrary.RandomBool`) :`false` -360 :`true` 360))
      (bind (_direction _alpha) (`Timeline|Shoot_Rotate_Timeline` :!via `PlayFromStart`)
        (:`Update`
          (`SceneComponent.K2_SetRelativeRotation` (`self.Ray_1_Sphere`) (`KismetMathLibrary.MakeRotator` (* (`self.Attack_Rotate_Dir`) _alpha)) false false))))))

(event `TryShoot`
  ;[1 1 1] Shooting
  ;;[1 1 1] Trying
  (if (!= (`KismetMathLibrary.VSize` (`self.Hit_Location`)) 0.0)
    (`/Engine/EditorBlueprintResources/StandardMacros.DoOnce` false :!label _label_2
      (:`Completed`
        (`self.Shoot` (`self.Shoot_Angle`))
        (`KismetSystemLibrary.Delay` (`self.Attack_Interval`))
        (goto _label_2 :!via `Reset`)))))

(fn `UserConstructionScript`
  (`parent.UserConstructionScript`))