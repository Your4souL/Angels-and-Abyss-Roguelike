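; Player avatar character, exposing events that callers use to turn its mesh and make it jump.
; Avatar_Look_Foolow_Cursor applies a supplied rotator to the mesh's relative rotation, and Jump_Event calls the built-in Jump.
; Forward and right move events are marked obsolete and left empty, with their AddMovementInput logic and a RoguelikeController cast left disconnected.
; Tick and the construction script do nothing.
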(event `Avatar_Look_Foolow_Cursor`
  (params (Rotator :type "Rotator Structure"))
  (`SceneComponent.K2_SetRelativeRotation` (`self.Mesh`) Rotator false false))

(event `self.ReceiveTick`
  (params (DeltaSeconds :type "Float (single-precision)")))

(event `Move_Fwd`
  (params (Rotator :type "Rotator Structure") (Axis :type "Float (double-precision)"))
  ;[1 1 1] OBSOLETE Avatar Moving
)

(event `Move_Rgt`
  (params (Rotator :type "Rotator Structure") (Axis :type "Float (double-precision)"))
  ;[1 1 1] OBSOLETE Avatar Moving
)

(event `Jump_Event`
  (`self.Jump`))

(fn `UserConstructionScript`)