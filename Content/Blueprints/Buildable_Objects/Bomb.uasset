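; Buildable bomb that, on press activation, spawns an explosion scaled to its radius, damages Abyss_Hand actors within AimDistance, then destroys itself.
; Initiate pulses four scene components with phase-offset sine waves driven by the root mesh's animation position, with amplitude varying by PressTimer.
; Upgrade uses a FlipFlop to alternate between two tiers, each revealing extra eye components and setting AimDistance; the second also moves the fuse (Fitil).
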(event `self.Press_Activation`
  (bind _returnvalue (/ (- (`self.Aim_Distance`) 50.0) 100.0))
  (`NiagaraFunctionLibrary.SpawnSystemAtLocation` "/Game/Effects/Explosion/Explosion.Explosion" (`SceneComponent.K2_GetComponentLocation` (`self.Eye`)) (struct) (`KismetMathLibrary.MakeVector` _returnvalue _returnvalue _returnvalue))
  (bind _outactors (`GameplayStatics.GetAllActorsOfClass` "/Game/Blueprints/Abyss/Abyss_Hand.Abyss_Hand_C"))
  (for _array_element _outactors
    (if (<= (`self.GetDistanceTo` _array_element self) (`self.Aim_Distance`))
      (`/Game/Blueprints/Abyss/Abyss_Hand.Take_Damage` _array_element (0.0 0.0 0.0) "NewEnumerator0" 20)))
  (`self.K2_DestroyActor`))

(event `self.OnInvoke`
  (`parent.OnInvoke`)
  ;[1 1 1] Invoke Animations
  (`KismetSystemLibrary.Delay` 0.6))

(event `self.OnExile`
  (`parent.OnExile`))

(event `self.Initiate`
  (bind _returnvalue (- (`self.Pulsating_Scale`) (* (`self.Press_Timer`) 14.0)))
  (bind _returnvalue_2 (* -1080 (/ (`SkeletalMeshComponent.GetPosition` (`self.RootMesh`)) 2.58)))
  (bind _returnvalue_3 (/ (+ (`KismetMathLibrary.DegSin` _returnvalue_2) _returnvalue) _returnvalue))
  (bind _returnvalue_4 (/ (+ (`KismetMathLibrary.DegSin` (+ _returnvalue_2 135.0)) _returnvalue) _returnvalue))
  (bind _returnvalue_5 (/ (+ (`KismetMathLibrary.DegSin` (+ _returnvalue_2 180.0)) _returnvalue) _returnvalue))
  (bind _returnvalue_6 (/ (+ (`KismetMathLibrary.DegSin` (+ _returnvalue_2 45.0)) _returnvalue) _returnvalue))
  ;[1 1 1] initiate cycle
  (`SceneComponent.SetRelativeScale3D` (`self.Scale_Scene_1`) (`KismetMathLibrary.MakeVector` _returnvalue_3 _returnvalue_3 _returnvalue_3))
  (`SceneComponent.SetRelativeScale3D` (`self.Scale_Scene_2`) (`KismetMathLibrary.MakeVector` _returnvalue_6 _returnvalue_6 _returnvalue_6))
  (`SceneComponent.SetRelativeScale3D` (`self.Scale_Scene_3`) (`KismetMathLibrary.MakeVector` _returnvalue_4 _returnvalue_4 _returnvalue_4))
  (`SceneComponent.SetRelativeScale3D` (`self.Scale_Scene_4`) (`KismetMathLibrary.MakeVector` _returnvalue_5 _returnvalue_5 _returnvalue_5))
  (`parent.Initiate`))

(event `self.Upgrade`
  (`parent.Upgrade`)
  (`/Engine/EditorBlueprintResources/StandardMacros.FlipFlop`
    (:`A`
      (`SceneComponent.SetVisibility` (`self.Eye_lvl2_1`) true false)
      (`SceneComponent.SetVisibility` (`self.Eye_lvl2_2`) true false)
      (`SceneComponent.SetVisibility` (`self.Eye_lvl2_3`) true false)
      (set `self.Aim_Distance` 450.0))
    (:`B`
      (`SceneComponent.SetVisibility` (`self.Eye_lvl3_1`) true false)
      (`SceneComponent.SetVisibility` (`self.Eye_lvl3_2`) true false)
      (`SceneComponent.SetVisibility` (`self.Eye_lvl3_3`) true false)
      (`SceneComponent.SetVisibility` (`self.Eye_lvl3_4`) true false)
      (`SceneComponent.SetVisibility` (`self.Eye_lvl3_5`) true false)
      (`SceneComponent.K2_SetRelativeLocation` (`self.Fitil`) (-43.0 7.0 -10.0) false false)
      (set `self.Aim_Distance` 650.0))))

(fn `UserConstructionScript`
  (`parent.UserConstructionScript`))