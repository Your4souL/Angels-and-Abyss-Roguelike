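; Base Blueprint for buildable Angels in the roguelike, handling summoning, floating, upgrades up to level 3, damage and exile.
; A curve timeline flies the mesh in, then reverses on exile to free its blocks and destroy it after a partial Flame refund.
; A self-recalling Delay loop drives sine bobbing and the button's hold-progress material, firing the empty PressActivation hook when full.
; Upgrades spend Flame, while lethal damage frees blocks immediately.
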(event `Invoke_Effect`
  (`NiagaraFunctionLibrary.SpawnSystemAtLocation` "/Game/Effects/Angel_Invoke.Angel_Invoke" (- (`SceneComponent.K2_GetComponentLocation` (`self.DefaultSceneRoot`)) (0.0 0.0 60.0)))
  (`KismetSystemLibrary.Delay` 2.58)
  (`self.Invoke_Effect`))

(event `OnInvoke`
  (bind _asinvisible_button (cast `/Game/Interface/InvisibleButton` (`WidgetComponent.GetWidget` (`self.Button`)) :!pure true))
  ;[1 1 1] Invoke
  (set `/Game/Interface/InvisibleButton.Owner` self _asinvisible_button)
  (bind _returnvalue (`Image.GetDynamicMaterial` (`/Game/Interface/InvisibleButton.Progress` _asinvisible_button)))
  (set `self.Press_Confirmation_Material` _returnvalue)
  (`TimelineComponent.SetPlayRate` (`self.Invoke_TM`) 3.0)
  (`self.Invoke_Effect`)
  (bind (_direction _flycurve) (`Timeline|Invoke_TM` :!via `PlayFromStart` :!label _label)
    (:`Update`
      (`SceneComponent.K2_SetRelativeLocation` (`self.RootMesh`) (`KismetMathLibrary.MakeVector` (* 5 (.x _flycurve)) (* 5 (.y _flycurve)) (* (`self.Invoke_Z_Scale`) (.z _flycurve))) false false))
    (:`Finished`
      (switch `ETimelineDirection` _direction
        (:`Forward`
          (`KismetSystemLibrary.Delay` 0.0)
          (`self.Initiate`)
          (`SceneComponent.SetVisibility` (`self.Button`) true false))
        (:`Backward`
          (for _array_element (`self.Blocks`)
            (`/Game/Blueprints/Block.Set_Avilibility` _array_element true))
          (`self.K2_DestroyActor`))))))

(event `OnExile`
  (bind _lvl (`self.Lvl`))
  (bind _asroguelike_controller (cast `/Game/Blueprints/RoguelikeController` (`GameplayStatics.GetPlayerController` 0) :!pure true))
  ;[1 1 1] Invoke
  (`KismetArrayLibrary.Array_RemoveItem` (`/Game/Blueprints/RoguelikeController.Angels_Limit` _asroguelike_controller) self)
  (`/Game/Blueprints/RoguelikeController.Give_Flame` _asroguelike_controller (/ (* (`self.Cost`) (+ _lvl (`KismetMathLibrary.Conv_BoolToInt` (== _lvl 3)))) 2))
  (set `self.Active` false)
  (goto _label :!via `ReverseFromEnd`))

(event `Press_Activation`)

(event `Initiate`
  (bind _press_timer (`self.Press_Timer`))
  ;[1 1 1] Initiate
  (`self.Floating`)
  (`KismetSystemLibrary.Delay` 0.016)
  (`MaterialInstanceDynamic.SetScalarParameterValue` (`self.Press_Confirmation_Material`) "Alpha" _press_timer)
  (bind _output_get (set `self.Press_Timer` (`KismetMathLibrary.FClamp` (+ _press_timer (`self.Press_Iterator`)) 0.0 1.1)))
  (if (== _output_get 1.1)
    (`self.Press_Activation`)
    (`/Engine/EditorBlueprintResources/StandardMacros.IsValid` self
      (:`Is Valid`
        _)))
  (if (`self.Active`)
    (`self.Initiate`)))

(event `Try_Upgrade`
  (if (< (`self.Lvl`) 3)
    (`self.Upgrade`)))

(event `Floating`
  (bind _rootmesh (`self.RootMesh`))
  ;[1 1 1] Floating
  (`SceneComponent.K2_SetRelativeLocation` _rootmesh (`KismetMathLibrary.MakeVector` 0.0 0.0 (+ (`self.Floating_Offset`) (* (`self.Floating_Scale`) (`KismetMathLibrary.DegSin` (* -360 (/ (`SkeletalMeshComponent.GetPosition` _rootmesh) 2.58)))))) false false))

(event `Upgrade`
  (bind _lvl (`self.Lvl`))
  (bind _asroguelike_controller (cast `/Game/Blueprints/RoguelikeController` (`GameplayStatics.GetPlayerController` 0)))
  (`/Game/Blueprints/RoguelikeController.Give_Flame` _asroguelike_controller (* (`self.Cost`) _lvl -1))
  (`/Engine/EditorBlueprintResources/StandardMacros.IncrementInt` _lvl
    (:`  `
      (if (`/Game/Blueprints/RoguelikeController.Tutorial` _asroguelike_controller)
        (`/Engine/EditorBlueprintResources/StandardMacros.DoOnce` false
          (:`Completed`
            (`/Game/Interface/Tutorial_Slides.Hide_After_Upgrade` (`/Game/Blueprints/RoguelikeController.Tutorial_Ref` _asroguelike_controller))))))))

(event `Take Damage`
  (params (Damage :type Integer))
  (bind _output_get (set `self.Hp` (- (`self.Hp`) Damage)))
  (`NiagaraFunctionLibrary.SpawnSystemAtLocation` "/Game/Effects/Abyss_Massive_Burst.Abyss_Massive_Burst" (`SceneComponent.K2_GetComponentLocation` (`self.RootMesh`)))
  (if (<= _output_get 0)
    (for _array_element (`self.Blocks`)
      (`/Game/Blueprints/Block.Set_Avilibility` _array_element true))
    (`KismetArrayLibrary.Array_RemoveItem` (`/Game/Blueprints/RoguelikeController.Angels_Limit` (cast `/Game/Blueprints/RoguelikeController` (`GameplayStatics.GetPlayerController` 0) :!pure true)) self)
    (`self.K2_DestroyActor`)))

(fn `UserConstructionScript`)