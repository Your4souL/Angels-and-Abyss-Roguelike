(event `self.ReceiveBeginPlay`
  ;[1 1 1] Begin play Settings
  (bind _returnvalue (`|CreateWidget` "/Game/Interface/GUI.GUI_C" self))
  (bind _output_get (set `self.GUI_Ref` _returnvalue))
  (`UserWidget.AddToViewport` _output_get 0)
  (bind _outactors (`GameplayStatics.GetAllActorsOfClassWithTag` "/Game/Blueprints/BlockGridGenerator.BlockGridGenerator_C" "Main_Level_Generator"))
  (bind _output (`|GetArrayItem` _outactors))
  (set `self.Island_Controller` _output)
  (bind _output_get_2 (set `self.Field_Center` (`SceneComponent.K2_GetComponentLocation` (`/Game/Blueprints/BlockGridGenerator.Plain` _output))))
  (`|ExecutionSequence`
    (:`then_0`
      (bind _returnvalue_2 (`|SpawnActorFromClass` "/Script/Engine.DirectionalLight" (`KismetMathLibrary.MakeTransform` (+ _output_get_2 (0.0 0.0 1000.0) (-1410.0 -1410.0 0.0)) (struct :`Pitch` 10.0 :`Yaw` -45.0)) "Undefined" "OverrideRootScale" null null))
      (bind _output_get_3 (set `self.Main_Light` _returnvalue_2))
      (bind _lightcomponent (`Light.LightComponent` _output_get_3))
      (`LightComponent.SetIntensity` _lightcomponent 2.0)
      (`LightComponentBase.SetCastShadows` _lightcomponent false)
      (`SceneComponent.SetMobility` _lightcomponent "Movable")
      (`LightComponent.SetLightColor` _lightcomponent (struct :`R` 1.0 :`G` 0.37199 :`A` 1.0) true))
    (:`then_1`
      (bind _returnvalue_3 (`|SpawnActorFromClass` "/Script/Engine.CameraActor" (`KismetMathLibrary.MakeTransform` (+ _output_get_2 (0.0 0.0 1000.0) (-1410.0 -1410.0 0.0)) (struct :`Pitch` -45.0 :`Yaw` -45.0)) "Undefined" "OverrideRootScale" null null))
      (bind _output_get_4 (set `self.Main_Camera` _returnvalue_3))
      (`self.SetViewTargetWithBlend` _output_get_4)
      (`CameraComponent.SetFieldOfView` (`CameraActor.CameraComponent` _output_get_4) 70.0)
      (bind _returnvalue_4 (`|CreateWidget` "/Game/Interface/Build_Menu.Build_Menu_C" self))
      (set `self.Build_Menu_Ref` _returnvalue_4)
      (`self.Define_Abyss_Position` 0.5)
      (bind _returnvalue_5 (`|CreateWidget` "/Game/Interface/Upgrade_Menu.Upgrade_Menu_C" self))
      (set `self.Upgrade_Menu_Ref` _returnvalue_5)
      (`self.Initiate`))))

(event `Cancel_Build`
  (bind _build_position_block (`self.Build_Position_Block`))
  ;[1 1 1 1 40] Tower control
  ;;[1 1 1 1 40] Interface tower build menu
  (`Widget.RemoveFromParent` (`self.Build_Menu_Ref`))
  (`Widget.RemoveFromParent` (`self.Upgrade_Menu_Ref`))
  (`/Engine/EditorBlueprintResources/StandardMacros.IsValid` _build_position_block
    (:`Is Valid`
      (`/Game/Blueprints/Block.Force_Deselect` _build_position_block))
    (:`Is Not Valid`
      _))
  (set `self.Build_Position_Block` null)
  (set `self.Tower_to_Upgrade` null))

(event `InputAction|Click`
  (params (Key :type "Key Structure"))
  ;[1 1 1 1 40] Tower control
  ;;[1 1 1 1 40] Interface tower build menu
  (:`Pressed`
    (`self.Cancel_Build`)))

(event `Build_Slot`
  (params (Slot :type Integer))
  (bind _build_position_block (`self.Build_Position_Block`))
  ;[1 1 1 1 40] Tower control
  ;;[1 1 1 1 40] Build Angel
  (if (>= (`self.Flame`) 5)
    (set `self.Flame` (- (`self.Flame`) 5))
    (bind _returnvalue (`|SpawnActorFromClass` "/Game/Blueprints/Buildable_Objects/Legioneer.Legioneer_C" (`KismetMathLibrary.MakeTransform` (+ (`self.K2_GetActorLocation` _build_position_block) (0.0 0.0 200.0)) (struct) (3.0 3.0 3.0)) "Undefined" "OverrideRootScale" null null))
    (`/Game/Blueprints/Buildable_Objects/AngelBase.OnInvoke` _returnvalue)
    (set `/Game/Blueprints/Block.Occupied` true _build_position_block)
    (`PrimitiveComponent.SetMaterial` (`/Game/Blueprints/Block.BlockMesh` _build_position_block) 0 "/Game/Meshes/_Materials/Cubes/AngelFullCubeMat.AngelFullCubeMat")
    (`self.Cancel_Build`)
    (else
      (`/Game/Interface/GUI.PlayCantBuild` (`self.GUI_Ref`)))))

(event `Key|Two`
  (params (Key :type "Key Structure"))
  ;[1 1 1] Debug Test Commands
  (:`Pressed`
    (bind _returnvalue (`GameplayStatics.GetActorOfClass` "/Game/Blueprints/Abyss/Abyss_Spawner.Abyss_Spawner_C"))
    (`/Engine/EditorBlueprintResources/StandardMacros.DoOnce` false :!label _label
      (:`Completed`
        (bind _result (`/Engine/EditorBlueprintResources/StandardMacros.IncrementInt` (`self.Wave_Number`))
          (:`  `
            (`/Game/Blueprints/Abyss/Abyss_Spawner.Start_Wave` _returnvalue _result)))))))

(event `InputAction|Call_Menu`
  (params (Key :type "Key Structure"))
  (bind _build_menu_ref (`self.Build_Menu_Ref`))
  ;[1 1 1 1 40] Tower control
  ;;[1 1 1 1 40] Interface tower build menu
  (:`Pressed`
    (`Widget.RemoveFromParent` (`self.Build_Menu_Ref`))
    (`Widget.RemoveFromParent` (`self.Upgrade_Menu_Ref`))
    (bind _asblock (cast `/Game/Blueprints/Block` (`.HitActor` (`GameplayStatics.BreakHitResult` (`self.GetHitResultUnderCursorByChannel` "TraceTypeQuery2")))))
    (if (not (`/Game/Blueprints/Block.Z_covered` _asblock))
      (bind _output_get (set `self.Build_Position_Block` _asblock))
      (if (not (`/Game/Blueprints/Block.Occupied` _asblock))
        (`/Game/Blueprints/Block.Force_Select` _output_get)
        (`UserWidget.AddToViewport` _build_menu_ref 0)
        (bind _screenposition (`GameplayStatics.ProjectWorldToScreen` self (`self.K2_GetActorLocation` _asblock)))
        (`UserWidget.SetPositionInViewport` _build_menu_ref (`KismetMathLibrary.MakeVector2D` (- (`KismetMathLibrary.BreakVector2D` _screenposition) 300.0) (- (`.Y` (`KismetMathLibrary.BreakVector2D` _screenposition)) 400.0)) true)))))

(event `Key|One`
  (params (Key :type "Key Structure"))
  ;[1 1 1] Debug Test Commands
  (:`Pressed`
    (`GameplayStatics.OpenLevel` "Level_Map")))

(event `Key|Three`
  (params (Key :type "Key Structure"))
  ;[1 1 1] Debug Test Commands
  (:`Pressed`
    (goto _label :!via `Reset`)))

(event `Upgrade_Base`
  ;[1 1 1 1 40] Tower control
  (`/Game/Blueprints/WingedBase.Upgrade` (`self.Base_to_Upgrade`)))

(event `Show_Base_Upgrade_Menu`
  (bind _upgrade_menu_ref (`self.Upgrade_Menu_Ref`))
  (bind _screenposition (`GameplayStatics.ProjectWorldToScreen` self (`self.K2_GetActorLocation` (`self.Base_to_Upgrade`))))
  ;[1 1 1 1 40] Tower control
  ;;[1 1 1] Call upgrade menues
  (`self.Cancel_Build`)
  (`UserWidget.AddToViewport` _upgrade_menu_ref 0)
  (`UserWidget.SetPositionInViewport` _upgrade_menu_ref (`KismetMathLibrary.MakeVector2D` (- (`KismetMathLibrary.BreakVector2D` _screenposition) 300.0) (- (`.Y` (`KismetMathLibrary.BreakVector2D` _screenposition)) 200.0)) true))

(event `Upgrade_Tower`
  (bind _tower_to_upgrade (`self.Tower_to_Upgrade`))
  ;[1 1 1 1 40] Tower control
  (if (>= (`self.Flame`) (* (`/Game/Blueprints/Buildable_Objects/AngelBase.Lvl` _tower_to_upgrade) 5))
    (`/Game/Blueprints/Buildable_Objects/AngelBase.Try_Upgrade` _tower_to_upgrade)
    (else
      (`/Game/Interface/GUI.PlayCantBuild` (`self.GUI_Ref`)))))

(event `Show_Tower_Upgrade_Menu`
  (params (Tower :type "/Game/Blueprints/Buildable_Objects/AngelBase Object Reference"))
  (bind _upgrade_menu_ref (`self.Upgrade_Menu_Ref`))
  (bind _screenposition (`GameplayStatics.ProjectWorldToScreen` self (`self.K2_GetActorLocation` (`self.Tower_to_Upgrade`))))
  ;[1 1 1 1 40] Tower control
  ;;[1 1 1] Call upgrade menues
  (`self.Cancel_Build`)
  (set `self.Tower_to_Upgrade` Tower)
  (`UserWidget.AddToViewport` _upgrade_menu_ref 0)
  (`UserWidget.SetPositionInViewport` _upgrade_menu_ref (`KismetMathLibrary.MakeVector2D` (- (`KismetMathLibrary.BreakVector2D` _screenposition) 300.0) (- (`.Y` (`KismetMathLibrary.BreakVector2D` _screenposition)) 200.0)) true))

(event `Initiate`
  (bind _base_to_upgrade (`self.Base_to_Upgrade`))
  ;[1 1 1] Initiate Updates
  (bind _summmass (`/Game/Blueprints/BlockGridGenerator.Get_Island_Mass` (`self.Island_Controller`)))
  (bind _returnvalue (- _summmass (`/Game/Blueprints/WingedBase.Wing_Power` _base_to_upgrade)))
  (bind _returnvalue_2 (/ _returnvalue -1000000.0))
  (set `self.Fall_Speed` _returnvalue_2)
  (bind _output_get (set `self.Current_Island_Height` (`KismetMathLibrary.FMin` 1.0 (`KismetMathLibrary.FMax` 0.0 (+ (`self.Current_Island_Height`) _returnvalue_2)))))
  (`self.Define_Abyss_Position` _output_get)
  (for _array_element (`/Game/Blueprints/BlockGridGenerator.Blocks_Array` (`self.Island_Controller`))
    (`/Game/Blueprints/Block.Update_Falling_System` _array_element (`self.View_Angle`) (`KismetMathLibrary.FClamp` (/ _returnvalue (* 100 (`/Game/Blueprints/WingedBase.Wing_Power_Multiplyer` _base_to_upgrade))) -1.0)))
  (`KismetSystemLibrary.Delay` 0.016)
  (`self.Initiate`))

(event `InputAxis|Rotate_Camera_isometric`
  (params (AxisValue :type "Float (single-precision)"))
  (bind _main_camera (`self.Main_Camera`))
  (bind _field_center (`self.Field_Center`))
  (bind (_view_angle_roll _view_angle_pitch _view_angle_yaw) (`KismetMathLibrary.BreakRotator` (`self.View_Angle`)))
  (bind _returnvalue (+ (`KismetMathLibrary.GreaterGreater_VectorRotator` (3000.0 0.0 0.0) (`self.View_Angle`)) _field_center (0.0 0.0 3000.0)))
  ;[1 1 1 1 40] Camera Control
  (if (!= AxisValue 0.0)
    (`self.Cancel_Build`))
  (set `self.View_Angle` (`KismetMathLibrary.MakeRotator` 0.0 0.0 (+ _view_angle_yaw AxisValue)))
  (`self.K2_SetActorLocation` _main_camera _returnvalue false false)
  (`self.K2_SetActorRotation` _main_camera (`KismetMathLibrary.FindLookAtRotation` _returnvalue (+ _field_center (0.0 0.0 300.0))) false))

(event `Define_Abyss_Position`
  (params (Pos :type "Float (double-precision)"))
  (bind (_returnvalue_x _returnvalue_y) (`KismetMathLibrary.BreakVector` (`SceneComponent.K2_GetComponentLocation` (`/Game/Blueprints/BlockGridGenerator.Plain` (`self.Island_Controller`)))))
  ;[1 1 1] Initiate Updates
  (bind _output_get (set `self.Current_Island_Height` Pos))
  (bind _returnvalue (`GameplayStatics.GetActorOfClass` "/Game/Blueprints/Abyss/Abyss_Spawner.Abyss_Spawner_C"))
  (`self.K2_SetActorLocation` _returnvalue (`KismetMathLibrary.MakeVector` _returnvalue_x _returnvalue_y (`KismetMathLibrary.Lerp` -2200.0 -8700.0 _output_get)) false false))

(fn `UserConstructionScript`)